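; Active skill Blueprint that casts a fire spread from the owning player in the direction they face.
; On the server, a successful parent launch spawns the fire emitter and a BP_FireSpread actor at the player's location, aligned to control yaw.
; The spawned actor receives the owner plus damage from skill power and a fraction of player power, and is set to overlap collision.
; Leveling up raises the skill's power and energy cost.
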(event `self.ReceiveBeginPlay`)

(event `self.ReceiveActorBeginOverlap`
  (params (OtherActor :type "Actor Object Reference")))

(event `self.ReceiveTick`
  (params (DeltaSeconds :type "Float (single-precision)"))
  (`parent.ReceiveTick` 0.0))

(fn `LaunchSkill`
  (returns (launched :type Boolean))
  (bind _playerowner (`self.playerOwner`))
  (bind _returnvalue (`self.K2_GetActorLocation` _playerowner))
  (bind _returnvalue_2 (`KismetMathLibrary.MakeRot` 0.0 (.yaw (`Pawn.GetControlRotation` _playerowner))))
  (`/Engine/EditorBlueprintResources/ActorMacros.Switch Has Authority`
    (:`Authority`
      (bind _launched (`parent.LaunchSkill`))
      (if _launched
        (`GameplayStatics.SpawnEmitterAtLocation` "/Game/Assets/PS_Spells/PS_FireSpread.PS_FireSpread" _returnvalue _returnvalue_2)
        (bind _returnvalue_3 (`|SpawnActorFromClass` "/Game/Sources/Skills/ActiveSkills/BP_FireSpread.BP_FireSpread_C" (`KismetMathLibrary.MakeTransform` _returnvalue _returnvalue_2) true))
        (bind _asbp_fire_spread (cast `/Game/Sources/Skills/ActiveSkills/BP_FireSpread` _returnvalue_3)
          (:`then`
            (`/Game/Sources/Skills/ActiveSkills/BP_FireSpread.Initialize` _asbp_fire_spread (`self.playerOwner`) (+ (`KismetMathLibrary.FFloor` (* (`/Game/Sources/BP_ABaseCharacter.GetPower` (`self.playerOwner`)) 0.2)) (`self.power`)))
            (`PrimitiveComponent.SetCollisionProfileName` _asbp_fire_spread "OverlapAllDynamic"))
          (:`CastFailed`
            _))
        (return _launched)))))

(fn `LevelUp`
  (returns (hasLevelUp :type Boolean))
  (bind _haslevelup (`parent.LevelUp`))
  (set `self.power` (+ (`self.power`) 20))
  (set `self.energyCost` (+ (`self.energyCost`) 20))
  (return _haslevelup))

(fn `UserConstructionScript`
  (`parent.UserConstructionScript`))