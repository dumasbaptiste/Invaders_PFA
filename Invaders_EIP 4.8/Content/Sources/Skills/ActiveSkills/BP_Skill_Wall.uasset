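; BP_Skill_Wall is an active skill that places a wall in front of the player who uses it.
; Its LaunchSkill override calls the parent implementation, then spawns a BP_Wall a fixed distance along the owner's forward vector, matching the owner's rotation.
; It returns the parent's result but does not check it, so the wall spawns regardless of that value.
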(event `self.ReceiveBeginPlay`)

(event `self.ReceiveActorBeginOverlap`
  (params (OtherActor :type "Actor Object Reference")))

(event `self.ReceiveTick`
  (params (DeltaSeconds :type "Float (single-precision)"))
  (`parent.ReceiveTick` 0.0))

(fn `LaunchSkill`
  (returns (launched :type Boolean))
  (bind _playerowner (`self.playerOwner`))
  (bind _launched (`parent.LaunchSkill`))
  (`|SpawnActorFromClass` "/Game/Sources/Skills/ActiveSkills/BP_Wall.BP_Wall_C" (`KismetMathLibrary.MakeTransform` (+ (`self.K2_GetActorLocation` _playerowner) (* (`self.GetActorForwardVector` _playerowner) 600.0)) (`self.K2_GetActorRotation` _playerowner)))
  (return _launched))

(fn `UserConstructionScript`
  (`parent.UserConstructionScript`))