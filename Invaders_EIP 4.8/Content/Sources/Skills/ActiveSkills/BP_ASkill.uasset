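; Generic active skill for a player, holding its stats, display info, cooldown and level.
; Tick counts the cooldown down, and TestSkillLaunching requires enough energy, no cooldown and an unmuted owner.
; LaunchSkill sets the cooldown scaled by the owner's reduction without spending energy; it, cooldown edits and level-ups are authority-only.
; SetCanBeLvlUp grants pending upgrades at player-level thresholds up to five, clearing them when the owner cannot upgrade.
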(event `self.ReceiveTick`
  (params (DeltaSeconds :type "Float (single-precision)"))
  (if (>= (`self.cooldown`) 0.0)
    (set `self.cooldown` (- (`self.cooldown`) DeltaSeconds))
    (else
      (set `self.cooldown` -1.0))))

(fn `Add to ActualCooldown`
  (params (toAdd :type "Float (double-precision)") (`resetCooldown ?` :type Boolean))
  (`/Engine/EditorBlueprintResources/ActorMacros.Switch Has Authority`
    (:`Authority`
      (if `resetCooldown ?`
        (set `self.cooldown` 0.0)
        (else
          (set `self.cooldown` (+ toAdd (`self.cooldown`))))))))

(fn `Get Image`
  (returns (Value :type "SlateBrush Structure"))
  (return (`self.Image`)))

(fn `GetActualCooldown`
  (returns (cooldown :type "Float (double-precision)"))
  (return (`self.cooldown`)))

(fn `GetBaseCooldown`
  (returns (cooldown :type "Float (double-precision)"))
  (return (`self.baseCooldown`)))

(fn `GetCanBeLvlUp`
  (returns (CanBeLvlUp :type Boolean))
  (return (> (`self.CanBeLvlUp`) 0)))

(fn `GetDescription`
  (returns (description :type String))
  (return (`self.description`)))

(fn `GetLevel`
  (returns (level :type Integer))
  (return (`self.level`)))

(fn `GetManaCost`
  (returns (manaCost :type Integer))
  (return (`self.energyCost`)))

(fn `GetName`
  (returns (name :type String))
  (return (`self.name`)))

(fn `GetPower`
  (returns (power :type Integer))
  (return (`self.power`)))

(fn `GetRange`
  (returns (range :type Integer))
  (return (`self.range`)))

(fn `IsTrueDamage`
  (returns (isTrueDamage :type Boolean))
  (return (`self.bIsTrueDamage`)))

(fn `LaunchSkill`
  (returns (launched :type Boolean))
  (`/Engine/EditorBlueprintResources/ActorMacros.Switch Has Authority`
    (:`Authority`
      (set `self.cooldown` (* (- 1.0 (`/Game/Sources/Avatar/BP_AAvatar.GetCooldownReduction` (`self.playerOwner`))) (`self.baseCooldown`)))
      (return true))
    (:`Remote`
      (`KismetSystemLibrary.PrintString` "You're on the client"))))

(fn `LevelUp`
  (returns (hasLevelUp :type Boolean))
  (`/Engine/EditorBlueprintResources/ActorMacros.Switch Has Authority`
    (:`Authority`
      (bind _output_get (set `self.level` (+ (`self.level`) 1)))
      (set `self.CanBeLvlUp` (- (`self.CanBeLvlUp`) 1))
      (`KismetSystemLibrary.PrintString` (`KismetStringLibrary.Conv_IntToString` _output_get))
      (return false))))

(fn `SetCanBeLvlUp`
  (params (PlayerLevel :type Integer :default 0) (isPPUse :type Boolean :default false))
  (if isPPUse
    (if (<= (`/Game/Sources/Avatar/BP_AAvatar.GetCanLvlUpSkill` (`self.playerOwner`)) 0)
      (set `self.CanBeLvlUp` 0))
    (elif (< (+ (`self.level`) (`self.CanBeLvlUp`)) 5)
      (if (and (>= PlayerLevel (`KismetArrayLibrary.Array_Get` (`self.LvlPlayerCanLevelUp`) (+ (`self.level`) (`self.CanBeLvlUp`)))) (< (`self.level`) 5))
        (set `self.CanBeLvlUp` (+ (`self.CanBeLvlUp`) 1))))))

(fn `SetPlayerOwner`
  (params (playerOwner :type "/Game/Sources/Avatar/BP_AAvatar Object Reference"))
  (set `self.playerOwner` playerOwner))

(fn `TestSkillLaunching`
  (returns (canBeLaunch :type Boolean))
  (bind _playerowner (`self.playerOwner`))
  (return (and (>= (`/Game/Sources/BP_ABaseCharacter.getEnergyPoints` _playerowner) (`self.energyCost`)) (<= (`self.cooldown`) 0.0) (not (`/Game/Sources/BP_ABaseCharacter.isMute` _playerowner)))))

(fn `UserConstructionScript`)