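; BP_Skill_FireRing is an active skill that creates a fire ring at the owning player's location.
; LaunchSkill runs the parent implementation, prints a debug message, then spawns a BP_FireRing actor facing the player's control yaw, with pitch and roll zeroed.
; It initializes the spawned ring with the player owner and returns the parent's launch result.
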(fn `LaunchSkill`
  (returns (launched :type Boolean))
  (bind _playerowner (`self.playerOwner`))
  (bind _launched (`parent.LaunchSkill`))
  (`KismetSystemLibrary.PrintString` "Skill Launched !")
  (bind _returnvalue (`|SpawnActorFromClass` "/Game/Sources/Skills/ActiveSkills/BP_FireRing.BP_FireRing_C" (`KismetMathLibrary.MakeTransform` (`self.K2_GetActorLocation` _playerowner) (`KismetMathLibrary.MakeRot` 0.0 (.yaw (`Pawn.GetControlRotation` _playerowner))))))
  (bind _asbp_fire_ring (cast `/Game/Sources/Skills/ActiveSkills/BP_FireRing` _returnvalue))
  (`/Game/Sources/Skills/ActiveSkills/BP_FireRing.Initialize` _asbp_fire_ring (`self.playerOwner`))
  (return _launched))

(fn `UserConstructionScript`
  (`parent.UserConstructionScript`))