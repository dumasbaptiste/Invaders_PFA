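; Active skill that summons a fire pillar actor at the owning player's position.
; LaunchSkill runs the parent launch logic, then spawns BP_FirePillar at the player's transform and returns the parent's result.
; The pillar is initialized with the owner, the skill's range, and the skill's power plus a small floored share of the player's power.
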(event `self.ReceiveBeginPlay`)

(event `self.ReceiveActorBeginOverlap`
  (params (OtherActor :type "Actor Object Reference")))

(event `self.ReceiveTick`
  (params (DeltaSeconds :type "Float (single-precision)"))
  (`parent.ReceiveTick` 0.0))

(fn `LaunchSkill`
  (returns (launched :type Boolean))
  (bind _playerowner (`self.playerOwner`))
  (bind _launched (`parent.LaunchSkill`))
  (bind _returnvalue (`|SpawnActorFromClass` "/Game/Sources/Skills/ActiveSkills/BP_FirePillar.BP_FirePillar_C" (`self.GetTransform` _playerowner)))
  (`/Game/Sources/Skills/ActiveSkills/BP_FirePillar.Initialize` _returnvalue _playerowner (+ (`self.power`) (`KismetMathLibrary.FFloor` (* (`/Game/Sources/BP_ABaseCharacter.GetPower` _playerowner) 0.05))) (`self.range`))
  (return _launched))

(fn `UserConstructionScript`
  (`parent.UserConstructionScript`))