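; BP_FireRing is a short-lived active-skill actor that repeatedly damages enemy characters inside its collider.
; Initialize stores the owning player, whose team filters out allies and whose power scales the damage on top of a flat base.
; On BeginPlay, a looping timer polls the collider's overlapping characters to apply damage, and a second timer destroys the actor when its lifetime ends.
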(event `DealDamages`
  (bind _playerowner (`self.playerOwner`))
  (for _array_element (`PrimitiveComponent.GetOverlappingActors` (`self.Collider`) "/Game/Sources/BP_ABaseCharacter.BP_ABaseCharacter_C")
    (bind _asbp_abase_character (cast `/Game/Sources/BP_ABaseCharacter` _array_element))
    (if (!= (`/Game/Sources/BP_ABaseCharacter.team` _asbp_abase_character) (`/Game/Sources/BP_ABaseCharacter.team` _playerowner))
      (`/Game/Sources/BP_ABaseCharacter.TakeDamages` _asbp_abase_character false "NewEnumerator1" false (`KismetMathLibrary.FFloor` (+ (* (`/Game/Sources/BP_ABaseCharacter.GetPower` _playerowner) 0.05) 10.0)) _playerowner))))

(event `End`
  (`self.K2_DestroyActor`))

(event `self.ReceiveBeginPlay`
  (`KismetSystemLibrary.K2_SetTimer` null "End" 5.0)
  (`KismetSystemLibrary.K2_SetTimerDelegate` (delegate `DealDamages`) 0.5 true))

(event `self.ReceiveActorBeginOverlap`
  (params (OtherActor :type "Actor Object Reference")))

(event `self.ReceiveTick`
  (params (DeltaSeconds :type "Float (single-precision)")))

(fn `Initialize`
  (params (playerOwner :type "/Game/Sources/Avatar/BP_AAvatar Object Reference"))
  (set `self.playerOwner` playerOwner))

(fn `UserConstructionScript`)