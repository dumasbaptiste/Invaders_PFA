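; BP_FirePillar is an active skill actor that rains fire pillars around its owning player for five seconds, then destroys itself.
; A looping timer recenters it on the owner and randomly targets either accumulated enemy positions, with X and Y rolled independently, or a random point in range, also the fallback without enemies.
; Each pillar spawns a BP_FirePillar_PS, while only the authority sphere-traces there to damage opposing-team characters.
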(event `ChoosePlace`
  (bind _returnvalue (`self.K2_GetActorLocation`))
  (bind _atrange (`self.atRange`))
  (bind _range (`self.range`))
  (bind _x (.x (`self.K2_GetActorLocation`)))
  (bind _y (.y (`self.K2_GetActorLocation`)))
  (`self.K2_SetActorLocation` (`self.K2_GetActorLocation` (`self.playerOwner`)))
  (if (> (`KismetMathLibrary.RandomInteger` 100) 50)
    (bind _outhits (`KismetSystemLibrary.SphereTraceMultiForObjects` _returnvalue (+ _returnvalue (0.0 0.0 250.0)) (`KismetMathLibrary.Conv_IntToDouble` (`self.range`)) (`self.desiredObjectTypes`) false (`|MakeArray` (`self.playerOwner`))))
    (for _array_element _outhits
      (bind _asbp_abase_character (cast `/Game/Sources/BP_ABaseCharacter` (`.HitActor` (`GameplayStatics.BreakHitResult` _array_element))))
      (if (!= (`/Game/Sources/BP_ABaseCharacter.team` _asbp_abase_character) (`/Game/Sources/BP_ABaseCharacter.team` (`self.playerOwner`)))
        (`KismetArrayLibrary.Array_AddUnique` (`self.atRange`) _asbp_abase_character)))
    (if (> (`KismetArrayLibrary.Array_Length` (`self.atRange`)) 0)
      (`self.CreatePillars` (`KismetMathLibrary.MakeVector` (.x (`self.K2_GetActorLocation` (`KismetArrayLibrary.Array_Get` _atrange (`KismetMathLibrary.RandomInteger` (`KismetArrayLibrary.Array_Length` _atrange))))) (.y (`self.K2_GetActorLocation` (`KismetArrayLibrary.Array_Get` _atrange (`KismetMathLibrary.RandomInteger` (`KismetArrayLibrary.Array_Length` _atrange))))) 100.0))
      (else
        (`self.NobodyAround`)))
    (else
      (`self.CreatePillars` (`KismetMathLibrary.MakeVector` (`KismetMathLibrary.RandomFloatInRange` (- _x (`KismetMathLibrary.Conv_IntToDouble` _range)) (+ _x (`KismetMathLibrary.Conv_IntToDouble` _range))) (`KismetMathLibrary.RandomFloatInRange` (- _y (`KismetMathLibrary.Conv_IntToDouble` _range)) (+ _y (`KismetMathLibrary.Conv_IntToDouble` _range))) 100.0) :!label _label))))

(event `NobodyAround`
  (goto _label))

(event `CreatePillars`
  (params (position :type "Object.Vector Structure"))
  (`|ExecutionSequence`
    (:`then_0`
      (`|SpawnActorFromClass` "/Game/Sources/Skills/ActiveSkills/BP_FirePillar_PS.BP_FirePillar_PS_C" (`KismetMathLibrary.Conv_VectorToTransform` position) true))
    (:`then_1`
      (`/Engine/EditorBlueprintResources/ActorMacros.Switch Has Authority`
        (:`Authority`
          (bind _outhits (`KismetSystemLibrary.SphereTraceMultiForObjects` position (+ position (0.0 0.0 150.0)) 50.0 (`self.desiredObjectTypes`) false (`|MakeArray` (`self.playerOwner`) :!type "Actor Object Reference")))
          (for _array_element _outhits
            (bind _asbp_abase_character (cast `/Game/Sources/BP_ABaseCharacter` (`.HitActor` (`GameplayStatics.BreakHitResult` _array_element))))
            (if (!= (`/Game/Sources/BP_ABaseCharacter.team` _asbp_abase_character) (`/Game/Sources/BP_ABaseCharacter.team` (`self.playerOwner`)))
              (`/Game/Sources/BP_ABaseCharacter.TakeDamages` _asbp_abase_character false "NewEnumerator1" false (`self.power`) (`self.playerOwner`)))))))))

(event `setTimers`
  (`KismetSystemLibrary.K2_SetTimerDelegate` (delegate `ChoosePlace`) 0.25 true)
  (`KismetSystemLibrary.K2_SetTimerDelegate` (delegate `End`) 5.0))

(event `End`
  (`self.K2_DestroyActor`))

(fn `Initialize`
  (params (playerOwner :type "/Game/Sources/Avatar/BP_AAvatar Object Reference") (power :type Integer) (range :type Integer))
  (set `self.playerOwner` playerOwner)
  (set `self.power` power)
  (set `self.range` range)
  (`self.setTimers`))

(fn `UserConstructionScript`)