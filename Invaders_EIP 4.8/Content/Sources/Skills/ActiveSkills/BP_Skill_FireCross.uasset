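; Active skill Blueprint that casts a fire cross centered on the owning player.
; LaunchSkill spawns four BP_FireWall actors at the player's location, yawed in quarter turns from the player's rotation so they form a cross.
; It then passes the player owner to each wall and returns true.
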(event `self.ReceiveBeginPlay`)

(event `self.ReceiveActorBeginOverlap`
  (params (OtherActor :type "Actor Object Reference")))

(event `self.ReceiveTick`
  (params (DeltaSeconds :type "Float (single-precision)"))
  (`parent.ReceiveTick` 0.0))

(fn `LaunchSkill`
  (returns (launched :type Boolean))
  (bind _playerowner (`self.playerOwner`))
  (bind _location (.location (`self.GetTransform` _playerowner)))
  (bind _rotation (.rotation (`self.GetTransform` _playerowner)))
  (bind _returnvalue (`|SpawnActorFromClass` "/Game/Sources/Skills/ActiveSkills/BP_FireWall.BP_FireWall_C" (`KismetMathLibrary.MakeTransform` _location _rotation)))
  (bind _returnvalue_2 (`|SpawnActorFromClass` "/Game/Sources/Skills/ActiveSkills/BP_FireWall.BP_FireWall_C" (`KismetMathLibrary.MakeTransform` _location (`KismetMathLibrary.MakeRot` (.pitch _rotation) (+ (.yaw _rotation) 90.0) (.roll _rotation)))))
  (bind _returnvalue_3 (`|SpawnActorFromClass` "/Game/Sources/Skills/ActiveSkills/BP_FireWall.BP_FireWall_C" (`KismetMathLibrary.MakeTransform` _location (`KismetMathLibrary.MakeRot` (.pitch _rotation) (+ (.yaw _rotation) 180.0) (.roll _rotation)))))
  (bind _returnvalue_4 (`|SpawnActorFromClass` "/Game/Sources/Skills/ActiveSkills/BP_FireWall.BP_FireWall_C" (`KismetMathLibrary.MakeTransform` _location (`KismetMathLibrary.MakeRot` (.pitch _rotation) (+ (.yaw _rotation) 270.0) (.roll _rotation)))))
  (`/Game/Sources/Skills/ActiveSkills/BP_FireWall.SetPlayerOwner` _returnvalue_4 _playerowner)
  (`/Game/Sources/Skills/ActiveSkills/BP_FireWall.SetPlayerOwner` _returnvalue_2 _playerowner)
  (`/Game/Sources/Skills/ActiveSkills/BP_FireWall.SetPlayerOwner` _returnvalue_3 _playerowner)
  (`/Game/Sources/Skills/ActiveSkills/BP_FireWall.SetPlayerOwner` _returnvalue _playerowner)
  (return true))

(fn `UserConstructionScript`
  (`parent.UserConstructionScript`))