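; BP_FireWall is an active-skill fire wall actor that deals periodic area damage and destroys itself after a few seconds.
; A looping timer runs Damage each second, hitting every character overlapping its Trigger through TakeDamages, credited to PlayerOwner.
; A team comparison against the owner is present, but both branches are empty, so allies are damaged too.
; SetPlayerOwner assigns the owning player.
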(event `End`
  (`self.K2_DestroyActor`))

(event `self.ReceiveBeginPlay`
  (`KismetSystemLibrary.K2_SetTimer` null "End" 5.0)
  (`KismetSystemLibrary.K2_SetTimer` null "Damage" 1.0 true))

(event `self.ReceiveActorBeginOverlap`
  (params (OtherActor :type "Actor Object Reference")))

(event `self.ReceiveTick`
  (params (DeltaSeconds :type "Float (single-precision)")))

(fn `Damage`
  (bind _playerowner (`self.PlayerOwner`))
  (for _array_element (`PrimitiveComponent.GetOverlappingActors` (`self.Trigger`) "/Game/Sources/BP_ABaseCharacter.BP_ABaseCharacter_C")
    (bind _asbp_abase_character (cast `/Game/Sources/BP_ABaseCharacter` _array_element))
    (if (!= (`/Game/Sources/BP_ABaseCharacter.team` _asbp_abase_character) (`/Game/Sources/BP_ABaseCharacter.team` _playerowner))
      _
      (else
        _))
    (`/Game/Sources/BP_ABaseCharacter.TakeDamages` _asbp_abase_character false "NewEnumerator1" false 50 _playerowner)))

(fn `SetPlayerOwner`
  (params (Set :type "/Game/Sources/Avatar/BP_AAvatar Object Reference"))
  (set `self.PlayerOwner` Set))

(fn `UserConstructionScript`)