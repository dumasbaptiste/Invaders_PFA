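; BP_FireSpread is a short-lived fire skill actor that damages enemy characters in a forward-moving area.
; Tick pushes the Collider along the actor's forward vector, and each overlapped character on another team takes damage only once, credited to PlayerOwner.
; Initialize sets owner and damage on authority only.
; A timed FlipFlop removes a component (apparently the Collider) first, then destroys the actor after a further delay.
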(event `delete`
  (`/Engine/EditorBlueprintResources/StandardMacros.FlipFlop`
    (:`A`
      (`ActorComponent.K2_DestroyComponent`)
      (`KismetSystemLibrary.K2_SetTimerDelegate` (delegate `delete`) 1.25))
    (:`B`
      (`self.K2_DestroyActor`))))

(event `self.ReceiveBeginPlay`
  (`KismetSystemLibrary.K2_SetTimerDelegate` (delegate `delete`) 0.75))

(event `self.ReceiveActorBeginOverlap`
  (params (OtherActor :type "Actor Object Reference"))
  (bind _hitten (`self.hitten`))
  (bind _playerowner (`self.playerOwner`))
  (bind _asbp_abase_character (cast `/Game/Sources/BP_ABaseCharacter` OtherActor))
  (if (and (not (`KismetArrayLibrary.Array_Contains` _hitten _asbp_abase_character)) (!= (`/Game/Sources/BP_ABaseCharacter.team` _asbp_abase_character) (`/Game/Sources/BP_ABaseCharacter.team` _playerowner)))
    (`KismetArrayLibrary.Array_AddUnique` _hitten _asbp_abase_character)
    (`/Game/Sources/BP_ABaseCharacter.TakeDamages` _asbp_abase_character false "NewEnumerator1" false (`self.damages`) _playerowner)))

(event `self.ReceiveTick`
  (params (DeltaSeconds :type "Float (single-precision)"))
  (bind _collider (`self.Collider`))
  (`/Engine/EditorBlueprintResources/StandardMacros.IsValid` _collider
    (:`Is Valid`
      (`SceneComponent.K2_SetWorldLocation` _collider (+ (* (`self.GetActorForwardVector`) (* DeltaSeconds 600.0)) (`SceneComponent.K2_GetComponentLocation` _collider)) false))))

(fn `Initialize`
  (params (playerOwnerValue :type "/Game/Sources/Avatar/BP_AAvatar Object Reference") (damages :type Integer))
  (`/Engine/EditorBlueprintResources/ActorMacros.Switch Has Authority`
    (:`Authority`
      (set `self.playerOwner` playerOwnerValue)
      (set `self.damages` damages))))

(fn `UserConstructionScript`)