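; Minion base attack projectile that damages the first character it hits on an opposing team.
; On hit it runs the parent logic, then, if the owner is valid and the first hit target's team differs, applies fixed damage credited to the owner.
; Both a successful hit and the Finish event flag the projectile to auto-destroy when finished, extending the parent projectile's behavior.
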(fn `Finish`
  (returns (return :type Boolean))
  (`parent.Finish`)
  (set `self.bAutoDestroyWhenFinished` true)
  (return false))

(fn `OnHit`
  (returns (return :type Boolean))
  (bind _hitten (`self.hitten`))
  (bind _ownercharacter (`self.ownerCharacter`))
  (bind _item (`KismetArrayLibrary.Array_Get` _hitten))
  (`parent.OnHit`)
  (`/Engine/EditorBlueprintResources/StandardMacros.IsValid` _ownercharacter
    (:`Is Valid`
      (if (> (`KismetArrayLibrary.Array_Length` _hitten) 0)
        (if (!= (`/Game/Sources/BP_ABaseCharacter.team` _ownercharacter) (`/Game/Sources/BP_ABaseCharacter.team` _item))
          (`/Game/Sources/BP_ABaseCharacter.TakeDamages` _item false "NewEnumerator0" false 10 (`self.ownerCharacter`))
          (set `self.bAutoDestroyWhenFinished` true)
          (return false))))))

(fn `UserConstructionScript`
  (`parent.UserConstructionScript`))