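; Base projectile actor that flies straight along its forward vector, covering its Range over a set duration.
; Initialize sets duration, range and owner on authority, and Tick drives an authority-only Update until Finish flags it done.
; Each step line-traces the upcoming movement on the Camera channel, ignoring the owner, to avoid tunneling.
; Hit characters are gathered in Hitten for the stub OnHit hook, then cleared; a helper picks damage type.
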(event EventTick
  (params (DeltaSeconds :type Float%20%28single-precision%29))
  ;[1 1 1] Update the projectile, making him go forward
  (CallFunction|Update DeltaSeconds))

(fn ConstructionScript)

(fn Initialize
  (params (duration :type Float%20%28single-precision%29) (range :type Integer) (owner :type BP%20A%20Base%20Character%20Object%20Reference))
  (Networking|SwitchHasAuthority
    (:Authority
      (Variables|Default|SettotalDuration duration)
      (Variables|Default|Setrange range)
      (Variables|Default|SetownerCharacter owner)
      (return true))))

(fn Finish
  (bind _output_get (Variables|Default|SetbIsFinished true))
  (return _output_get))

(fn Update
  (params (deltaTime :type Float%20%28single-precision%29))
  (if (and (Ability|HasAuthority) (not (Variables|Default|GetbIsFinished)))
    (if (> (+ deltaTime (Variables|Default|GetactualTime)) (Variables|Default|GettotalDuration))
      (LocalVariables|SetdeltaTmp (- (Variables|Default|GettotalDuration) (Variables|Default|GetactualTime)))
      (Variables|Default|SetactualTime (Variables|Default|GettotalDuration))
      (else
        (LocalVariables|SetdeltaTmp deltaTime)
        (Variables|Default|SetactualTime (+ (LocalVariables|GetdeltaTmp) (Variables|Default|GetactualTime)))))
    (bind (_outhits _returnvalue) (Class|KismetSystemLibrary|LineTraceMultiNEW (Transformation|GetActorLocation) (+ (* (Transformation|GetActorForwardVector) (* (/ (Math|Conversions|ToFloat(Integer) (Variables|Default|Getrange)) (Variables|Default|GettotalDuration)) (LocalVariables|GetdeltaTmp))) (Transformation|GetActorLocation)) "TraceTypeQuery2" false (Utilities|Array|MakeArray (Variables|Default|GetownerCharacter)) "None" true)) ; Perform a raycast to see if an actor has been hitten since last frame
    (if _returnvalue
      ;[1 1 1] For Each hitten actors except the owner, put it into an array
      (for _array_element _outhits
        (bind _asbp_abase_character (Utilities|Casting|CastToBP_ABaseCharacter (.HitActor (Collision|BreakHitResult _array_element))))
        (Utilities|Array|AddUnique (Variables|Default|Gethitten) _asbp_abase_character))
      (CallFunction|OnHit)
      (Utilities|Array|Clear (Variables|Default|Gethitten)))
    (Transformation|SetActorLocation (+ (* (Transformation|GetActorForwardVector) (* (/ (Math|Conversions|ToFloat(Integer) (Variables|Default|Getrange)) (Variables|Default|GettotalDuration)) (LocalVariables|GetdeltaTmp))) (Transformation|GetActorLocation)) false)
    (if (>= (Variables|Default|GetactualTime) (Variables|Default|GettotalDuration))
      (CallFunction|Finish)
      (return true))))

(fn OnHit
  (return true))

(fn ChooseDamageType
  (params (isEnergetic :type Boolean))
  (if isEnergetic
    (LocalVariables|Setret "NewEnumerator1")
    (else
      (LocalVariables|Setret "NewEnumerator0")))
  (return (LocalVariables|Getret)))