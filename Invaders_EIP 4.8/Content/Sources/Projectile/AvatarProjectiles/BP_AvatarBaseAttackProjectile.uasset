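; Base projectile for avatar basic attacks, extending a parent projectile class through OnHit and Finish overrides.
; On hit, it damages the first hit target if that target is on a different team from a valid owner character, flagged as a basic attack.
; Damage amount comes from the owner's power and damage type from its energetic state.
; A damaging hit or Finish enables auto-destroy when finished.
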(fn `Finish`
  (returns (return :type Boolean))
  (`parent.Finish`)
  (set `self.bAutoDestroyWhenFinished` true)
  (return false))

(fn `OnHit`
  (returns (return :type Boolean))
  (bind _ownercharacter (`self.ownerCharacter`))
  (bind _hitten (`self.hitten`))
  (bind _ownercharacter_2 (`self.ownerCharacter`))
  (bind _item (`KismetArrayLibrary.Array_Get` _hitten))
  (`parent.OnHit`)
  (`/Engine/EditorBlueprintResources/StandardMacros.IsValid` _ownercharacter_2
    (:`Is Valid`
      (if (> (`KismetArrayLibrary.Array_Length` _hitten) 0)
        (if (!= (`/Game/Sources/BP_ABaseCharacter.team` _ownercharacter_2) (`/Game/Sources/BP_ABaseCharacter.team` _item))
          (`/Game/Sources/BP_ABaseCharacter.TakeDamages` _item false (`self.ChooseDamageType` (`/Game/Sources/BP_ABaseCharacter.bIsEnergetic` _ownercharacter)) true (`/Game/Sources/BP_ABaseCharacter.GetPower` _ownercharacter) _ownercharacter)
          (set `self.bAutoDestroyWhenFinished` true))))
    (:`Is Not Valid`
      _))
  (return false))

(fn `UserConstructionScript`
  (`parent.UserConstructionScript`))