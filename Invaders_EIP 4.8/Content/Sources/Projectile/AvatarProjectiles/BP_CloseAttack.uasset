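; BP_CloseAttack is a short-lived projectile that serves as an avatar's close-range basic attack.
; On Update it gathers characters overlapping its mesh except the owner, calls OnHit if any are found, then finishes and flags itself for auto-destruction.
; OnHit deals the owner's power as close-range damage to gathered characters on other teams and prints a debug string.
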(event `self.ReceiveBeginPlay`)

(event `self.ReceiveActorBeginOverlap`
  (params (OtherActor :type "Actor Object Reference")))

(event `self.ReceiveTick`
  (params (DeltaSeconds :type "Float (single-precision)"))
  (`parent.ReceiveTick` 0.0))

(fn `OnHit`
  (returns (return :type Boolean))
  (bind _ownercharacter (`self.ownerCharacter`))
  (bind _ownercharacter_2 (`self.ownerCharacter`))
  (`/Engine/EditorBlueprintResources/StandardMacros.IsValid` _ownercharacter
    (:`Is Valid`
      (for _array_element (`self.hitten`)
        (if (!= (`/Game/Sources/BP_ABaseCharacter.team` _array_element) (`/Game/Sources/BP_ABaseCharacter.team` _ownercharacter))
          (`/Game/Sources/BP_ABaseCharacter.TakeDamages` _array_element true "NewEnumerator0" true (`/Game/Sources/BP_ABaseCharacter.GetPower` _ownercharacter_2) _ownercharacter_2)))
      (`KismetSystemLibrary.PrintString` "DAMAGE")
      (return false))))

(fn `Update`
  (params (deltaTime :type "Float (double-precision)"))
  (returns (return :type Boolean))
  (for _array_element (`PrimitiveComponent.GetOverlappingActors` (`self.Mesh`) "/Game/Sources/BP_ABaseCharacter.BP_ABaseCharacter_C")
    (if (!= (`self.ownerCharacter`) _array_element)
      (bind _asbp_abase_character (cast `/Game/Sources/BP_ABaseCharacter` _array_element))
      (`KismetArrayLibrary.Array_Add` (`self.hitten`) _asbp_abase_character)))
  (if (> (`KismetArrayLibrary.Array_Length` (`self.hitten`)) 0)
    (`self.OnHit`))
  (`self.Finish`)
  (set `self.bAutoDestroyWhenFinished` true)
  (return false))

(fn `UserConstructionScript`
  (`parent.UserConstructionScript`))