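; BP_FireBall is an avatar fireball projectile that damages an opposing-team target and explodes.
; On authority, OnHit damages the first hit target using a base amount plus a share of the owner's Power, then calls Finish.
; Finish runs the parent logic and Explose, which removes a component and attaches an explosion particle system.
; Explose also starts an authority-only timer that destroys the actor after a short delay.
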(event `self.ReceiveBeginPlay`)

(event `self.ReceiveActorBeginOverlap`
  (params (OtherActor :type "Actor Object Reference")))

(event `self.ReceiveTick`
  (params (DeltaSeconds :type "Float (single-precision)"))
  (`parent.ReceiveTick` DeltaSeconds))

(event `Explose`
  (`ActorComponent.K2_DestroyComponent`)
  (bind _returnvalue (`AddComponent|Particle System Component_2263`))
  (`ParticleSystemComponent.SetTemplate` _returnvalue "/Game/Assets/PS_Spells/PS_Explosion.PS_Explosion")
  (`/Engine/EditorBlueprintResources/ActorMacros.Switch Has Authority`
    (:`Authority`
      (`KismetSystemLibrary.K2_SetTimer` null "Die" 2.0))))

(event `Die`
  (`self.K2_DestroyActor`))

(fn `Finish`
  (returns (return :type Boolean))
  (`parent.Finish`)
  (`self.Explose`)
  (set `self.bAutoDestroyWhenFinished` true)
  (return true))

(fn `OnHit`
  (returns (return :type Boolean))
  (bind _ownercharacter (`self.ownerCharacter`))
  (bind _item (`KismetArrayLibrary.Array_Get` (`self.hitten`)))
  (`/Engine/EditorBlueprintResources/ActorMacros.Switch Has Authority`
    (:`Authority`
      (if (!= (`/Game/Sources/BP_ABaseCharacter.team` _item) (`/Game/Sources/BP_ABaseCharacter.team` (`self.ownerCharacter`)))
        (`/Game/Sources/BP_ABaseCharacter.TakeDamages` _item false "NewEnumerator1" false (`KismetMathLibrary.FFloor` (+ (* (`/Game/Sources/BP_ABaseCharacter.GetPower` _ownercharacter) 0.2) 50.0)) _ownercharacter)
        (`self.Finish`)
        (return false)))))

(fn `UserConstructionScript`
  (`parent.UserConstructionScript`))