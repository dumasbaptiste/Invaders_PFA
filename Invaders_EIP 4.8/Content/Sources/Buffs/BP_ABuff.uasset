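; BP_ABuff is a base buff Blueprint that declares the gameplay event hooks a buff can react to.
; Hooks cover the player, nearby allies and enemies, ticking, skill launches, normal and critical hits given or taken, healing, and avatar or minion kills.
; Every hook is a stub returning false and the construction script is empty, so the asset acts as an interface-like parent with no behavior of its own.
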(fn `OnGiveCriticalHit`
  (params (Player :type "/Game/Sources/BP_ABaseCharacter Object Reference") (Ennemy :type "/Game/Sources/BP_ABaseCharacter Object Reference") (Projectile :type "/Game/Sources/Projectile/BP_AProjectile Object Reference"))
  (returns (Ok :type Boolean))
  (return false))

(fn `OnGiveEnnemyLaunchingSkill`
  (params (Player :type "/Game/Sources/BP_ABaseCharacter Object Reference") (Ennemy :type "/Game/Sources/BP_ABaseCharacter Object Reference") (Skill :type "/Game/Sources/Skills/ActiveSkills/BP_ASkill Object Reference"))
  (returns (Ok :type Boolean))
  (return false))

(fn `OnGiveHit`
  (params (Player :type "/Game/Sources/BP_ABaseCharacter Object Reference") (Ennemy :type "/Game/Sources/BP_ABaseCharacter Object Reference") (Projectile :type "/Game/Sources/Projectile/BP_AProjectile Object Reference"))
  (returns (Ok :type Boolean))
  (return false))

(fn `OnHealPlayer`
  (params (Player :type "/Game/Sources/BP_ABaseCharacter Object Reference") (Allies :type "Array of /Game/Sources/BP_ABaseCharacter Object Reference"))
  (returns (Ok :type Boolean))
  (return false))

(fn `OnKillAvatar`
  (params (Ennemy :type "/Game/Sources/Avatar/BP_AAvatar Object Reference"))
  (returns (Ok :type Boolean))
  (return false))

(fn `OnKillMinions`
  (params (Minion :type "/Game/Sources/Minions/BP_AMinion Object Reference"))
  (returns (Ok :type Boolean))
  (return false))

(fn `OnLaunchSkill`
  (params (Player :type "/Game/Sources/BP_ABaseCharacter Object Reference") (Skill :type "/Game/Sources/Skills/ActiveSkills/BP_ASkill Object Reference"))
  (returns (Ok :type Boolean))
  (return false))

(fn `OnNearbyAllies`
  (returns (Ok :type Boolean))
  (return false))

(fn `OnNearbyEnnemies`
  (returns (Ok :type Boolean))
  (return false))

(fn `OnPlayer`
  (params (Player :type "/Game/Sources/BP_ABaseCharacter Object Reference"))
  (returns (Ok :type Boolean))
  (return false))

(fn `OnTakeCriticalHit`
  (params (Player :type "/Game/Sources/BP_ABaseCharacter Object Reference") (Ennemy :type "/Game/Sources/BP_ABaseCharacter Object Reference") (Projectile :type "/Game/Sources/Projectile/BP_AProjectile Object Reference"))
  (returns (Ok :type Boolean))
  (return false))

(fn `OnTakeEnnemyLaunchingSkill`
  (params (Player :type "/Game/Sources/BP_ABaseCharacter Object Reference") (Ennemy :type "/Game/Sources/BP_ABaseCharacter Object Reference") (Skill :type "/Game/Sources/Skills/ActiveSkills/BP_ASkill Object Reference"))
  (returns (OK :type Boolean))
  (return false))

(fn `OnTakeHit`
  (params (Player :type "/Game/Sources/BP_ABaseCharacter Object Reference") (Ennemy :type "/Game/Sources/BP_ABaseCharacter Object Reference") (Projectile :type "/Game/Sources/Projectile/BP_AProjectile Object Reference"))
  (returns (Ok :type Boolean))
  (return false))

(fn `OnTick`
  (params (Player :type "/Game/Sources/BP_ABaseCharacter Object Reference"))
  (returns (Ok :type Boolean))
  (return false))

(fn `UserConstructionScript`)