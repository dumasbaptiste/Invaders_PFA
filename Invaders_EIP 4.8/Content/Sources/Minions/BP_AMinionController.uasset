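; AI controller for minions patrolling lane or jungle waypoints.
; Ten seconds after possession, it caches the minion, seeds BB_Minion with home and patrol pattern, builds its route, then runs BT_Minion.
; FindWaypoints gathers BP_Waypoints on the minion's path for its team, then the opposite side discovered through the position-zero waypoint.
; It writes starting waypoint, direction and state to the blackboard; lane minions count down, others count up from zero.
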(event EventOnPossess
  (params (PossessedPawn :type Pawn%20Object%20Reference))
  (if (not (Variables|Default|GetIsInitialized))
    (Utilities|FlowControl|Delay 1e+01)
    ;[1 1 1] Store Minion
    (bind _asbp_aminion (Utilities|Casting|CastToBP_AMinion (Pawn|GetControlledPawn)))
    (Variables|Default|SetAMinion _asbp_aminion)
    (CallFunction|Initialize)))

(fn ConstructionScript)

(fn Initialize
  ;[1 1 1] Begin
  ;[1 1 1] Use BlackBoard BB_Minion
  (Class|AIController|UseBlackboard "/Game/Sources/Minions/BB_Minion.BB_Minion")
  ;[1 1 1] Set Home Location
  (LocalVariables|SetBB_KeyName "HomeLocation")
  (AI|Components|Blackboard|SetValueasVector (AI|GetBlackboard self) (LocalVariables|GetBB_KeyName) (Transformation|GetActorLocation (Variables|Default|GetAMinion)))
  ;[1 1 1] Set PatrolPattern
  (LocalVariables|SetBB_KeyName "PatrolPattern")
  (AI|Components|Blackboard|SetValueasEnum (AI|GetBlackboard self) (LocalVariables|GetBB_KeyName) (Variables|/Game/Sources/Minions/BP_AMinion.BP_AMinion_C|GetpatrolPattern (Variables|Default|GetAMinion)))
  (Utilities|FlowControl|Sequence
    (:then_0
      (CallFunction|FindWaypoints))
    (:then_1
      (AI|RunBehaviorTree "/Game/Sources/Minions/BT_Minion.BT_Minion"))
    (:then_2
      (Variables|Default|SetIsInitialized true))))

(fn FindWaypoints
  ;[1 1 1] Begin
  ;[1 1 1] Retrieving Waypoints following Minion Pattern
  (switch Utilities|FlowControl|Switch|SwitchonE_PatrolPattern (Variables|/Game/Sources/Minions/BP_AMinion.BP_AMinion_C|GetpatrolPattern (Variables|Default|GetAMinion))
    (:NewEnumerator0
      ;[1 1 1] Set to Idle
      (bind _output_get (LocalVariables|SetMinionStateEnum "NewEnumerator0"))
      (AI|Components|Blackboard|SetValueasEnum (AI|GetBlackboard self) (LocalVariables|GetBB_KeyName) _output_get))
    (:NewEnumerator1
      ;[1 1 1] Set Waypoint Starting Side
      (bind _output_get_2 (LocalVariables|SetBB_KeyName "WaypointSideTag" :!label _label))
      (AI|Components|Blackboard|SetValueasEnum (AI|GetBlackboard self) _output_get_2 (Variables|/Game/Sources/BP_ABaseCharacter.BP_ABaseCharacter_C|Getteam (Variables|Default|GetAMinion)))
      ;[1 1 1] Get All Waypoints
      (bind _outactors (Actor|GetAllActorsOfClass "/Game/Sources/Minions/BP_Waypoint.BP_Waypoint_C"))
      ;[1 1 1] Minion's TEAM side - Check Waypoint Side and add to Waypoints Array
      (bind _array_element (Utilities|Array|ForEachLoopwithBreak _outactors)
        (:LoopBody
          (bind _asbp_waypoint (Utilities|Casting|CastToBP_Waypoint _array_element))
          (LocalVariables|SetWaypointRef _asbp_waypoint)
          (if (== (Variables|/Game/Sources/Minions/BP_AMinion.BP_AMinion_C|Getpath (Variables|Default|GetAMinion)) (Variables|/Game/Sources/Minions/BP_Waypoint.BP_Waypoint_C|Getlane (LocalVariables|GetWaypointRef))) ; Check Lane
            (bind _array_element_2 (Utilities|Array|ForEachLoopwithBreak (Variables|/Game/Sources/Minions/BP_Waypoint.BP_Waypoint_C|Getsides (LocalVariables|GetWaypointRef)) :!label _label_2)
              (:LoopBody
                (if (== _array_element_2 (Variables|/Game/Sources/BP_ABaseCharacter.BP_ABaseCharacter_C|Getteam (Variables|Default|GetAMinion))) ; Check Team Side
                  (LocalVariables|SetSameSide (== _array_element_2 (Variables|/Game/Sources/BP_ABaseCharacter.BP_ABaseCharacter_C|Getteam (Variables|Default|GetAMinion))))
                  (Utilities|Array|Add (Variables|Default|GetWaypoints) (LocalVariables|GetWaypointRef))
                  (if (== (Variables|/Game/Sources/Minions/BP_Waypoint.BP_Waypoint_C|Getposition (LocalVariables|GetWaypointRef)) 0)
                    (bind _array_element_3 (Utilities|Array|ForEachLoopwithBreak (Variables|/Game/Sources/Minions/BP_Waypoint.BP_Waypoint_C|Getsides (LocalVariables|GetWaypointRef)) :!label _label_3)
                      (:LoopBody
                        (if (!= _array_element_3 (Variables|/Game/Sources/BP_ABaseCharacter.BP_ABaseCharacter_C|Getteam (Variables|Default|GetAMinion)))
                          (LocalVariables|SetOtherSide _array_element_3)
                          (goto _label_3 Break)))
                      (:Completed
                        (goto _label_2 Break)))
                    (else
                      (goto _label_2 Break))))))))
        (:Completed
          ;[1 1 1] Check if there are other waypoints
          (if (!= (LocalVariables|GetOtherSide) (Variables|/Game/Sources/BP_ABaseCharacter.BP_ABaseCharacter_C|Getteam (Variables|Default|GetAMinion)))
            ;[1 1 1] Minion's ENEMY side - Check Waypoint Side and add to Waypoints Array
            (bind _array_element_4 (Utilities|Array|ForEachLoopwithBreak _outactors)
              (:LoopBody
                (bind _asbp_waypoint_2 (Utilities|Casting|CastToBP_Waypoint _array_element_4))
                (LocalVariables|SetWaypointRef _asbp_waypoint_2)
                (if (== (Variables|/Game/Sources/Minions/BP_AMinion.BP_AMinion_C|Getpath (Variables|Default|GetAMinion)) (Variables|/Game/Sources/Minions/BP_Waypoint.BP_Waypoint_C|Getlane (LocalVariables|GetWaypointRef))) ; Check Lane
                  (if (!= (Variables|/Game/Sources/Minions/BP_Waypoint.BP_Waypoint_C|Getposition (LocalVariables|GetWaypointRef)) 0)
                    (bind _array_element_5 (Utilities|Array|ForEachLoopwithBreak (Variables|/Game/Sources/Minions/BP_Waypoint.BP_Waypoint_C|Getsides (LocalVariables|GetWaypointRef)) :!label _label_4)
                      (:LoopBody
                        (if (== _array_element_5 (LocalVariables|GetOtherSide))
                          (LocalVariables|SetSameSide (== _array_element_5 (LocalVariables|GetOtherSide)))
                          (Utilities|Array|Add (Variables|Default|GetWaypoints) (LocalVariables|GetWaypointRef))
                          (goto _label_4 Break)))))))
              (:Completed
                ;[1 1 1] Set MaxWaypoint
                (LocalVariables|SetMaxWaypoints (- (Utilities|Array|Length (Variables|Default|GetWaypoints)) 1) :!label _label_5)
                (if (Utilities|Enum|Equal(Enum) (Variables|/Game/Sources/Minions/BP_AMinion.BP_AMinion_C|GetpatrolPattern (Variables|Default|GetAMinion)) "NewEnumerator1")
                  (LocalVariables|SetMaxWaypoints (/ (LocalVariables|GetMaxWaypoints) 2)))
                (bind _output_get_3 (LocalVariables|SetBB_KeyName "WaypointTotal"))
                (Class|BlackboardComponent|SetValueasInt (AI|GetBlackboard self) _output_get_3 (LocalVariables|GetMaxWaypoints))
                ;[1 1 1] Find the initial Waypoint
                (LocalVariables|SetPatrolPatternEnum "NewEnumerator1")
                (bind _array_element_6 (Utilities|Array|ForEachLoopwithBreak (Variables|Default|GetWaypoints) :!label _label_6)
                  (:LoopBody
                    (LocalVariables|SetstartingWaypoint (Math|Integer|SelectInt 0 (LocalVariables|GetMaxWaypoints) (!= (Variables|/Game/Sources/Minions/BP_AMinion.BP_AMinion_C|GetpatrolPattern (Variables|Default|GetAMinion)) (LocalVariables|GetPatrolPatternEnum))))
                    (if (Math|Boolean|ANDBoolean (and (== (Utilities|Array|Get(acopy) (Variables|/Game/Sources/Minions/BP_Waypoint.BP_Waypoint_C|Getsides _array_element_6)) (Utilities|Array|Get(acopy) (Variables|/Game/Sources/Minions/BP_Waypoint.BP_Waypoint_C|Getsides _array_element_6) 1)) (== (Utilities|Array|Get(acopy) (Variables|/Game/Sources/Minions/BP_Waypoint.BP_Waypoint_C|Getsides _array_element_6) 1) (Variables|/Game/Sources/BP_ABaseCharacter.BP_ABaseCharacter_C|Getteam (Variables|Default|GetAMinion)))) (== (Variables|/Game/Sources/Minions/BP_Waypoint.BP_Waypoint_C|Getlane _array_element_6) (Variables|/Game/Sources/Minions/BP_AMinion.BP_AMinion_C|Getpath (Variables|Default|GetAMinion))) (== (Variables|/Game/Sources/Minions/BP_Waypoint.BP_Waypoint_C|Getposition _array_element_6) (LocalVariables|GetstartingWaypoint)))
                      (LocalVariables|SetWaypointRef _array_element_6)
                      (goto _label_6 Break)))
                  (:Completed
                    (CallFunction|FindWaypointswithPosition (LocalVariables|GetstartingWaypoint) (Variables|/Game/Sources/BP_ABaseCharacter.BP_ABaseCharacter_C|Getteam (Variables|Default|GetAMinion)))
                    ;[1 1 1] Set Waypoint
                    (bind _output_get_4 (LocalVariables|SetBB_KeyName "Waypoint"))
                    (AI|Components|Blackboard|SetValueasObject (AI|GetBlackboard self) _output_get_4 (LocalVariables|GetWaypointRef))
                    ;[1 1 1] Set WaypointLocation
                    (bind _output_get_5 (LocalVariables|SetBB_KeyName "WaypointLocation"))
                    (AI|Components|Blackboard|SetValueasVector (AI|GetBlackboard self) _output_get_5 (Transformation|GetActorLocation (LocalVariables|GetWaypointRef)))
                    (bind _output_get_6 (LocalVariables|SetBB_KeyName "WaypointPosition"))
                    (Class|BlackboardComponent|SetValueasInt (AI|GetBlackboard self) _output_get_6 (Variables|/Game/Sources/Minions/BP_Waypoint.BP_Waypoint_C|Getposition (LocalVariables|GetWaypointRef)))
                    (LocalVariables|SetPatrolPatternEnum "NewEnumerator1")
                    ;[1 1 1] Set WaypointIncrement
                    (if (!= (Variables|/Game/Sources/Minions/BP_AMinion.BP_AMinion_C|GetpatrolPattern (Variables|Default|GetAMinion)) (LocalVariables|GetPatrolPatternEnum))
                      (LocalVariables|SetWIncrement 1)
                      (else
                        (LocalVariables|SetWIncrement -1)))
                    (bind _output_get_7 (LocalVariables|SetBB_KeyName "WaypointIncrement"))
                    (Class|BlackboardComponent|SetValueasInt (AI|GetBlackboard self) _output_get_7 (LocalVariables|GetWIncrement))
                    ;[1 1 1] Set MinionState
                    (LocalVariables|SetBB_KeyName "MinionState")
                    (if (> (LocalVariables|GetMaxWaypoints) 0)
                      (LocalVariables|SetMinionStateEnum "NewEnumerator4")
                      (else
                        (LocalVariables|SetMinionStateEnum "NewEnumerator0")))
                    (AI|Components|Blackboard|SetValueasEnum (AI|GetBlackboard self) (LocalVariables|GetBB_KeyName) (LocalVariables|GetMinionStateEnum))))))
            (else
              (goto _label_5))))))
    (:NewEnumerator2
      (goto _label))))

(fn FindWaypointswithPosition
  (params (Position :type Integer :default 0) (Side :type E_Team%20Enum :default "NewEnumerator0"))
  (LocalVariables|SetTeam Side)
  (LocalVariables|SetPos Position)
  ;[1 1 1] Check Waypoints
  (if (!= 0 (Utilities|Array|Length (Variables|Default|GetWaypoints)))
    ;[1 1 1] Find Waypoint
    (bind _array_element (Utilities|Array|ForEachLoopwithBreak (Variables|Default|GetWaypoints) :!label _label)
      (:LoopBody
        (bind _output_get (Variables|Default|SetRetWaypoint _array_element))
        (if (== (Variables|/Game/Sources/Minions/BP_Waypoint.BP_Waypoint_C|Getposition _output_get) (LocalVariables|GetPos))
          (bind _array_element_2 (Utilities|Array|ForEachLoopwithBreak (Variables|/Game/Sources/Minions/BP_Waypoint.BP_Waypoint_C|Getsides (Variables|Default|GetRetWaypoint)))
            (:LoopBody
              (if (== _array_element_2 (LocalVariables|GetTeam))
                (goto _label Break))))))
      (:Completed
        (return (Variables|Default|GetRetWaypoint))))))