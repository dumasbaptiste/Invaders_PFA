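; Behavior tree task that moves a minion toward its blackboard follow target until it is within its range minus an offset.
; On execute it caches the controller and pawn, sets the monster state on the blackboard and opens a gate.
; While the gate is open, Tick reissues AIMoveTo every frame.
; Only a successful move updates the state, finishes the task and closes the gate; failure is unhandled.
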(event `CloseGate`
  ;[1 1 1] Receive Close Event
  (goto _label :!via `Close`))

(event `self.ReceiveTick`
  (params (OwnerActor :type "Actor Object Reference") (DeltaSeconds :type "Float (single-precision)"))
  ;[1 1 1] Event Tick
  ;[1 1 1] MoveTo Target
  (`/Engine/EditorBlueprintResources/StandardMacros.Gate` true :!label _label
    (:`Exit`
      (`|AIMoveTo` (`self.Minion`) (0.0 0.0 0.0) (`BTFunctionLibrary.GetBlackboardValueAsActor` (`self.TargetToFollow`)) (- (`KismetMathLibrary.Conv_IntToDouble` (`/Game/Sources/BP_ABaseCharacter.GetRange` (`self.Minion`))) (`self.Offset`))
        (:`OnSuccess`
          ;[1 1 1] Set Monster's State
          (bind _output_get (set `self.State` "NewEnumerator2"))
          (`BTFunctionLibrary.SetBlackboardValueAsEnum` (`self.MonsterState`) _output_get)
          ;[1 1 1] Finish and Close
          (`self.FinishExecute` true)
          (`self.CloseGate`))))))

(event `self.ReceiveExecuteAI`
  (params (OwnerController :type "AIController Object Reference") (ControlledPawn :type "Pawn Object Reference"))
  ;[1 1 1] Begin
  ;[1 1 1] Initialize
  (bind _asbp_aminion_controller (cast `/Game/Sources/Minions/BP_AMinionController` OwnerController))
  (set `self.MinionController` _asbp_aminion_controller)
  (bind _asbp_aminion (cast `/Game/Sources/Minions/BP_AMinion` ControlledPawn))
  (set `self.Minion` _asbp_aminion)
  ;[1 1 1] Set Monster's State
  (bind _output_get (set `self.State` "NewEnumerator1"))
  (`BTFunctionLibrary.SetBlackboardValueAsEnum` (`self.MonsterState`) _output_get)
  (goto _label :!via `Open`))