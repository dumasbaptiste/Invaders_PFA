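; Behavior tree task that moves a minion to the waypoint actor stored in its blackboard.
; On execute it caches the controller and minion, writes a minion state, clears the target location and opens a gate.
; While open, the gate lets Tick reissue AI MoveTo every frame; success writes another state and finishes the task.
; A separate CloseGate event shuts the gate.
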(event `CloseGate`
  ;[1 1 1] Receive Close Event
  (goto _label :!via `Close`))

(event `self.ReceiveTick`
  (params (OwnerActor :type "Actor Object Reference") (DeltaSeconds :type "Float (single-precision)"))
  ;[1 1 1] Event Tick
  ;[1 1 1] MoveTo Waypoint
  (`/Engine/EditorBlueprintResources/StandardMacros.Gate` true :!label _label
    (:`Exit`
      (`|AIMoveTo` (`Controller.K2_GetPawn` (`self.MinionController`)) (0.0 0.0 0.0) (`BTFunctionLibrary.GetBlackboardValueAsActor` (`self.Waypoint`)) (`self.ErrorOffset`)
        (:`OnSuccess`
          ;[1 1 1] Set Monster's State
          (set `self.State` "NewEnumerator3")
          (`BTFunctionLibrary.SetBlackboardValueAsEnum` (`self.MinionState`) (`self.State`))
          ;[1 1 1] Finish and Close
          (`self.FinishExecute` true))))))

(event `self.ReceiveExecuteAI`
  (params (OwnerController :type "AIController Object Reference") (ControlledPawn :type "Pawn Object Reference"))
  ;[1 1 1] Begin
  ;[1 1 1] Store Controller
  (bind _asbp_aminion_controller (cast `/Game/Sources/Minions/BP_AMinionController` OwnerController))
  (set `self.MinionController` _asbp_aminion_controller)
  (bind _asbp_aminion (cast `/Game/Sources/Minions/BP_AMinion` ControlledPawn))
  (set `self.AMinion` _asbp_aminion)
  ;[1 1 1] Set Monster's State
  (set `self.State` "NewEnumerator4")
  (`BTFunctionLibrary.SetBlackboardValueAsEnum` (`self.MinionState`) (`self.State`))
  (`BTFunctionLibrary.ClearBlackboardValue` (`self.TargetLocation`))
  (goto _label :!via `Open`))