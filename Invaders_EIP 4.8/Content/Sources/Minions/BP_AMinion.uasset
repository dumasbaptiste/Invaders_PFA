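; BP_AMinion is a minion character that fires attacks and rewards gold and experience when killed.
; Die sphere-traces within GivingRange for avatars on the killer's team, paying the killer in full and allies divided by KillCoeff.
; Attack spawns and initializes a projectile facing the control yaw.
; Stat setters are server-only and clamp at zero, though SetXpAmount takes no input and always writes zero.
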(fn ConstructionScript
  (|CallParentFunction))

(fn GetAgroRange
  (return (Variables|Stats|GetagroRange)))

(fn SetAgroRange
  (params (agroRange :type Integer))
  (Networking|SwitchHasAuthority
    (:Authority
      (LocalVariables|SetnewAgroRange agroRange)
      (if (< (LocalVariables|GetnewAgroRange) 0)
        (Variables|Stats|SetagroRange 0)
        (else
          (Variables|Stats|SetagroRange (LocalVariables|GetnewAgroRange)))))
    (:Remote
      (Development|PrintString "Are you trying to cheat ? You're on the client" true true "(R=1.000000,G=0.000000,B=0.000000,A=1.000000)"))))

(fn GetXpAmount
  (return (Variables|Stats|GetxpAmount)))

(fn SetXpAmount
  (Networking|SwitchHasAuthority
    (:Authority
      (LocalVariables|SetnewXpAmount 0)
      (if (< (LocalVariables|GetnewXpAmount) 0)
        (Variables|Stats|SetxpAmount 0)
        (else
          (Variables|Stats|SetxpAmount (LocalVariables|GetnewXpAmount)))))
    (:Remote
      (Development|PrintString "Are you trying to cheat ? You're on the client" true true "(R=1.000000,G=0.000000,B=0.000000,A=1.000000)"))))

(fn GetGoldAmount
  (return (Variables|Stats|GetgoldAmount)))

(fn SetGoldAmount
  (params (goldAmount :type Integer))
  (Networking|SwitchHasAuthority
    (:Authority
      (LocalVariables|SetnewGoldAmount goldAmount)
      (if (< (LocalVariables|GetnewGoldAmount) 0)
        (Variables|Stats|SetgoldAmount 0)
        (else
          (Variables|Stats|SetgoldAmount (LocalVariables|GetnewGoldAmount)))))
    (:Remote
      (Development|PrintString "Are you trying to cheat ? You're on the client" true true "(R=1.000000,G=0.000000,B=0.000000,A=1.000000)"))))

(fn Die
  (params (killer :type BP%20A%20Base%20Character%20Object%20Reference))
  (bind _returnvalue (Transformation|GetActorLocation))
  (bind _output_get (LocalVariables|Setkillercharacter killer))
  (Development|PrintString "DIE POTATOE !")
  (|CallParentFunction _output_get)
  ;[1 1 1] Getting Actors within Minion's GivingRange
  (bind _outhits (Collision|MultiSphereTraceForObjects _returnvalue (+ _returnvalue "0, 0,15.000000") (Math|Conversions|ToFloat(Integer) (Variables|Default|GetgivingRange)) (Utilities|Array|MakeArray "ObjectTypeQuery3") false (Utilities|Array|MakeArray self) "None"))
  ;[1 1 1] Getting Actors from Killer's team
  (for _array_element _outhits
    (bind _asbp_aavatar (Utilities|Casting|CastToBP_AAvatar (.HitActor (Collision|BreakHitResult _array_element))))
    (if (== (Variables|/Game/Sources/BP_ABaseCharacter.BP_ABaseCharacter_C|Getteam _asbp_aavatar) (Variables|/Game/Sources/BP_ABaseCharacter.BP_ABaseCharacter_C|Getteam (LocalVariables|Getkillercharacter)))
      ;[1 1 1] Giving Gold and Exp
      (bind _asbp_aavatar_2 (Utilities|Casting|CastToBP_AAvatar _asbp_aavatar))
      (if (== _asbp_aavatar_2 (LocalVariables|Getkillercharacter))
        ;;[1 0.1598 0.1789] Killer - Need a Rework !
        (Default|AddGold _asbp_aavatar_2 (Variables|Stats|GetgoldAmount))
        (Default|AddExperience _asbp_aavatar_2 (Variables|Stats|GetxpAmount))
        (else
          ;;[1 1 1] Killer's allies
          (Default|AddGold _asbp_aavatar_2 (/ (Variables|Stats|GetgoldAmount) (Variables|Stats|GetkillCoeff)))
          (Default|AddExperience _asbp_aavatar_2 (/ (Variables|Stats|GetxpAmount) (Variables|Stats|GetkillCoeff)))))))
  (bind _output_get_2 (Variables|Default|SetbAutoDestroyWhenFinished true))
  (return _output_get_2))

(fn Attack
  (bind _returnvalue (Game|SpawnActorfromClass "/Game/Sources/Projectile/MinionProjectiles/BP_MinionBaseAttackProjectile.BP_MinionBaseAttackProjectile_C" (Math|Transform|MakeTransform (Transformation|GetActorLocation) (Class|KismetMathLibrary|MakeRot 0.0 (.Yaw (Class|KismetMathLibrary|BreakRot (Pawn|GetControlRotation :!class /Script/Engine.Pawn))) 0.0) "0.100000,0.100000,0.100000") true 0))
  (Default|Initialize _returnvalue 0.1 (Variables|Default|Getrange) self))