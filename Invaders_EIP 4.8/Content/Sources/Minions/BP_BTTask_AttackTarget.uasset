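; Behavior tree task that makes a minion auto-attack the character stored as its blackboard target.
; It sets the minion state and, once the cooldown has elapsed, resets it to the inverse of attack speed and clears the animation time.
; With a valid target it stops the minion, turns it toward the target and calls Attack.
; It finishes successfully after attacking or while on cooldown, but never finishes if the target is invalid.
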(event `self.ReceiveExecuteAI`
  (params (OwnerController :type "AIController Object Reference") (ControlledPawn :type "Pawn Object Reference"))
  (bind _minion (`self.minion`))
  (bind _returnvalue (`BTFunctionLibrary.GetBlackboardValueAsObject` (`self.TargetToFollow`)))
  ;[1 1 1] Begin
  ;[1 1 1] Initialization
  (bind _asbp_aminion_controller (cast `/Game/Sources/Minions/BP_AMinionController` OwnerController))
  (set `self.minionController` _asbp_aminion_controller)
  (bind _asbp_aminion (cast `/Game/Sources/Minions/BP_AMinion` ControlledPawn))
  (set `self.minion` _asbp_aminion)
  ;[1 1 1] Set Monster State
  (set `self.state` "NewEnumerator2")
  (`BTFunctionLibrary.SetBlackboardValueAsEnum` (`self.MinionState`) (`self.state`))
  ;[1 1 1] Check If Monster can attack
  (if (<= (`BTFunctionLibrary.GetBlackboardValueAsFloat` (`self.AutoAttackCooldown`)) 0.0)
    ;[1 1 1] Get AttackSpeed and Set AutoAttackCooldown - AutoAttackAnim
    (bind _asbp_aminion_2 (cast `/Game/Sources/Minions/BP_AMinion` (`Controller.K2_GetPawn` (`self.minionController`))))
    (`BTFunctionLibrary.SetBlackboardValueAsFloat` (`self.AutoAttackCooldown`) (/ 1.0 (`/Game/Sources/BP_ABaseCharacter.GetAttackSpeed` _asbp_aminion_2)))
    (`BTFunctionLibrary.SetBlackboardValueAsFloat` (`self.AnimationTime`))
    ;[1 1 1] Get And Check TargetToFollow
    (`/Engine/EditorBlueprintResources/StandardMacros.IsValid` _returnvalue
      (:`Is Valid`
        ;[1 1 1] Stop Minion Movement and Focus the player
        (bind _asbp_abase_character (cast `/Game/Sources/BP_ABaseCharacter` _returnvalue))
        (`MovementComponent.StopMovementImmediately` (`self.minion`))
        (`Actor.SetActorRotation` _minion (`KismetMathLibrary.MakeRot` (.pitch (`Actor.K2_GetActorRotation` (`self.minion`))) (.yaw (`KismetMathLibrary.FindLookAtRotation` (`Actor.K2_GetActorLocation` (`self.minion`)) (`Actor.K2_GetActorLocation` _asbp_abase_character))) (.roll (`KismetMathLibrary.FindLookAtRotation` (`Actor.K2_GetActorLocation` (`self.minion`)) (`Actor.K2_GetActorLocation` _asbp_abase_character)))))
        ;[1 1 1] Attack
        (`/Game/Sources/Minions/BP_AMinion.Attack` _minion)
        ;[1 1 1] Finish
        (`self.FinishExecute` true)))
    (else
      ;[1 1 1] Finish
      (`self.FinishExecute` true))))