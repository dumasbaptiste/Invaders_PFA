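; Behavior tree decorator that ticks down minion timers held in the Blackboard during its condition check.
; Helper functions cover taunt (also tracking target location), stun, attack animation and auto-attack cooldown, each subtracting world delta time.
; Only the auto-attack update is connected; the other three, with their SetExecution gating, never run.
; The cooldown result is unused, so the check returns true whenever the owner casts to BP_AMinionController.
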(fn UpdateTaunt
  (bind _taunttarget (Variables|Taunt|GettauntTarget))
  (bind _tauntduration (Variables|Taunt|GettauntDuration))
  (bind _returnvalue (AI|BehaviorTree|GetBlackboardValueasActor _taunttarget))
  ;[1 1 1] Update TauntDuration
  (if (> (Class|BTFunctionLibrary|GetBlackboardValueasFloat (Variables|Taunt|GettauntDuration)) 0.0)
    (Class|BTFunctionLibrary|SetBlackboardValueasFloat _tauntduration (- (Class|BTFunctionLibrary|GetBlackboardValueasFloat _tauntduration) (Variables|Default|GetdeltaTime)))
    ;[1 1 1] Check TauntDuration value
    (if (<= (Class|BTFunctionLibrary|GetBlackboardValueasFloat (Variables|Taunt|GettauntDuration)) 0.0)
      ;[1 1 1] If TauntDuration less than 0
      (Class|BTFunctionLibrary|SetBlackboardValueasObject (Variables|Taunt|GettauntTarget))
      (else
        (Utilities|IsValid _returnvalue
          (:Is%20Valid
            (AI|BehaviorTree|SetBlackboardValueasVector (Variables|Taunt|GettauntLocation) (Transformation|GetActorLocation _returnvalue))))))
    (return true)))

(fn UpdateAnimation
  ;[1 1 1] Update AutoAttack Anim
  (if (> (Class|BTFunctionLibrary|GetBlackboardValueasFloat (Variables|Animation|GetanimationDuration)) 0.0)
    (Class|BTFunctionLibrary|SetBlackboardValueasFloat (Variables|Animation|GetanimationDuration) (- (Class|BTFunctionLibrary|GetBlackboardValueasFloat (Variables|Animation|GetanimationDuration)) (Variables|Default|GetdeltaTime)))
    (LocalVariables|SetExecute false)
    (else
      (LocalVariables|SetExecute true)))
  (return (LocalVariables|GetExecute)))

(fn UpdateStun
  ;[1 1 1] Update Stun Duration
  (if (> (Class|BTFunctionLibrary|GetBlackboardValueasFloat (Variables|Stun|GetstunDuration)) 0.0)
    (Class|BTFunctionLibrary|SetBlackboardValueasFloat (Variables|Stun|GetstunDuration) (- (Class|BTFunctionLibrary|GetBlackboardValueasFloat (Variables|Stun|GetstunDuration)) (Variables|Default|GetdeltaTime)))
    (LocalVariables|SetExecute false)
    (else
      (LocalVariables|SetExecute true)))
  (return (LocalVariables|GetExecute)))

(fn PerformConditionCheck
  (params (OwnerActor :type Actor%20Object%20Reference))
  ;[1 1 1] Store Minion Controller
  (bind _asbp_aminion_controller (Utilities|Casting|CastToBP_AMinionController OwnerActor))
  (Variables|Default|SetminionController _asbp_aminion_controller)
  (Variables|Default|SetdeltaTime (Utilities|Time|GetWorldDeltaSeconds))
  (Variables|Default|SetallowExecution true)
  (Utilities|FlowControl|Sequence
    (:then_2
      (CallFunction|UpdateAutoAttack))
    (:then_4
      (return (Variables|Default|GetallowExecution)))))

(fn UpdateAutoAttack
  ;[1 1 1] Update AutoAttackCooldown
  (if (> (Class|BTFunctionLibrary|GetBlackboardValueasFloat (Variables|AutoAttack|GetAutoAttackCooldown)) 0.0)
    (Class|BTFunctionLibrary|SetBlackboardValueasFloat (Variables|AutoAttack|GetAutoAttackCooldown) (- (Class|BTFunctionLibrary|GetBlackboardValueasFloat (Variables|AutoAttack|GetAutoAttackCooldown)) (Variables|Default|GetdeltaTime)))
    (LocalVariables|Setexecution false)
    (else
      (LocalVariables|Setexecution true)))
  (return (LocalVariables|Getexecution)))