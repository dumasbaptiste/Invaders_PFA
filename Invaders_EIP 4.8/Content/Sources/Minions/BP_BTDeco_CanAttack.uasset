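; Behavior Tree decorator that decides whether a minion can attack its TargetToFollow blackboard actor.
; It line-traces on the Camera channel from minion to target and passes when the target is hit within the minion's range.
; Hits on projectiles, or on actors IsAEnnemy does not report as enemies, join a local ignore list and the trace repeats.
; Any other hit, or no blocking hit, fails the check.
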(fn PerformConditionCheckAI
  (params (OwnerController :type AI%20Controller%20Object%20Reference) (ControlledPawn :type Pawn%20Object%20Reference))
  (bind _targettofollow (Variables|Default|GettargetToFollow))
  (bind _returnvalue (AI|BehaviorTree|GetBlackboardValueasActor _targettofollow))
  (bind _returnvalue_2 (Transformation|GetActorLocation _returnvalue))
  ;[1 1 1] Init
  (bind _asbp_aminion_controller (Utilities|Casting|CastToBP_AMinionController OwnerController))
  (Variables|Default|SetminionController _asbp_aminion_controller)
  (bind _asbp_aminion (Utilities|Casting|CastToBP_AMinion ControlledPawn))
  (bind _output_get (Variables|Default|Setminion _asbp_aminion))
  (Utilities|Array|AddUnique (LocalVariables|GetNewLocalVar_0) _output_get)
  ;[1 1 1] Raycast and Check
  (bind _outhit (Collision|LineTraceByChannel (Transformation|GetActorLocation (Variables|Default|Getminion)) _returnvalue_2 "TraceTypeQuery2" false (LocalVariables|GetNewLocalVar_0) "None" :!label _label))
  (bind _output_get_2 (LocalVariables|SetHitResult _outhit))
  (if (.bBlockingHit (Collision|BreakHitResult _output_get_2))
    (if (and (== (.HitActor (Collision|BreakHitResult (LocalVariables|GetHitResult))) (AI|BehaviorTree|GetBlackboardValueasActor (Variables|Default|GettargetToFollow))) (>= (Math|Conversions|ToFloat(Integer) (Default|GetRange (Variables|Default|Getminion))) (Math|Vector|VectorLength (- _returnvalue_2 (Transformation|GetActorLocation (Variables|Default|Getminion))))))
      ;[1 1 1] CanAttack
      (LocalVariables|SetRetValue true)
      (else
        ;[1 1 1] Redo another Raycast if the previous hit a Projectile or a Monster
        (if (or (Actor|ActorHasTag (.HitActor (Collision|BreakHitResult (LocalVariables|GetHitResult))) "Projectile") (Math|Boolean|NotEqual(Boolean) (Utilities|IsAEnnemy (Variables|/Game/Sources/BP_ABaseCharacter.BP_ABaseCharacter_C|Getteam (Variables|Default|Getminion)) (.HitActor (Collision|BreakHitResult (LocalVariables|GetHitResult)))) true))
          (Utilities|Array|AddUnique (LocalVariables|GetNewLocalVar_0) (.HitActor (Collision|BreakHitResult (LocalVariables|GetHitResult))))
          (goto _label)
          (else
            ;[1 1 1] CannotAttack
            (LocalVariables|SetRetValue false :!label _label_2)))))
    (else
      (goto _label_2)))
  (return (LocalVariables|GetRetValue)))