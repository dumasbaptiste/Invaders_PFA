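; Behavior tree service that picks an aggro target for a minion on each AI tick.
; It sphere-traces for pawns within the minion's aggro range, splitting hits into enemy candidates and ignored actors such as projectiles and allies.
; Line traces on the Camera channel test visibility, keeping the nearest visible enemy.
; The result updates the blackboard's follow target, also setting state and location when a target is found.
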(event EventReceiveTickAI
  (params (OwnerController :type AI%20Controller%20Object%20Reference) (ControlledPawn :type Pawn%20Object%20Reference) (DeltaSeconds :type Float%20%28single-precision%29))
  ;[1 1 1] Begin
  ;[1 1 1] Store Controller
  (bind _asbp_aminion_controller (Utilities|Casting|CastToBP_AMinionController OwnerController))
  (Variables|Default|SetminionController _asbp_aminion_controller)
  (bind _asbp_aminion (Utilities|Casting|CastToBP_AMinion ControlledPawn))
  (Variables|Default|Setminion _asbp_aminion)
  ;[1 1 1] Reset variables
  (Variables|Default|SettargetActor 0)
  (Utilities|Array|Clear (Variables|Default|GetIgnoreActors))
  ;[1 1 1] Set Monster Location
  (Variables|Default|SetminionLocation (Transformation|GetActorLocation (Pawn|GetControlledPawn (Variables|Default|GetminionController))))
  ;[1 1 1] Detect Characters
  (bind _hitresults (CallFunction|DetectCharactersWithinARadius))
  ;[1 1 1] Cleanning Array
  (bind (_cleanedarray _actorstoignore) (CallFunction|CleanHitArray _hitresults))
  (Variables|Default|SetIgnoreActors _actorstoignore)
  (bind _array_element (Utilities|Array|ForEachLoopwithBreak _cleanedarray)
    (:LoopBody
      ;[1 1 1] Add self to IgnoreActors
      (Utilities|Array|Add (Variables|Default|GetIgnoreActors) (Pawn|GetControlledPawn (Variables|Default|GetminionController)))
      ;[1 1 1] Raycast to the Character
      (bind _outhit (Collision|LineTraceByChannel (Variables|Default|GetminionLocation) (Transformation|GetActorLocation (.HitActor (Collision|BreakHitResult _array_element))) "TraceTypeQuery2" false (Variables|Default|GetIgnoreActors) "ForOneFrame"))
      (if (== (.HitActor (Collision|BreakHitResult _outhit)) (.HitActor (Collision|BreakHitResult _array_element)))
        ;[1 1 1] Set TargetActor if not set
        (Utilities|IsValid (Variables|Default|GettargetActor)
          (:Is%20Valid
            ;[1 1 1] Set TargetActor to the nearest
            (if (not (> (Math|Vector|VectorLength (- (Variables|Default|GetminionLocation) (Transformation|GetActorLocation (.HitActor (Collision|BreakHitResult _outhit))))) (Math|Vector|VectorLength (- (Variables|Default|GetminionLocation) (Transformation|GetActorLocation (Variables|Default|GettargetActor))))))
              (Variables|Default|SettargetActor (.HitActor (Collision|BreakHitResult _outhit)))))
          (:Is%20Not%20Valid
            (Variables|Default|SettargetActor (.HitActor (Collision|BreakHitResult _outhit)))))
        (else
          ;[1 1 1] Redo another Raycast if the previous hit a Projectile or a teammate
          (if (or (Actor|ActorHasTag (.HitActor (Collision|BreakHitResult _outhit)) "Projectile") (Utilities|IsEnnemy (Variables|/Game/Sources/BP_ABaseCharacter.BP_ABaseCharacter_C|Getteam (Variables|Default|Getminion)) (.HitActor (Collision|BreakHitResult _outhit))))
            (Utilities|Array|Add (Variables|Default|GetIgnoreActors) (.HitActor (Collision|BreakHitResult _outhit)))))))
    (:Completed
      ;[1 1 1] End
      (CallFunction|SetBlackBoardValues))))

(fn DetectCharactersWithinARadius
  (bind _minioncontroller (Variables|Default|GetminionController))
  (bind _returnvalue (Pawn|GetControlledPawn _minioncontroller))
  ;[1 1 1] Detect Characters within a Radius
  (bind _asbp_aminion (Utilities|Casting|CastToBP_AMinion _returnvalue))
  (bind _outhits (Collision|MultiSphereTraceForObjects (Variables|Default|GetminionLocation) (+ (Variables|Default|GetminionLocation) "0, 0,15.000000") (Math|Conversions|ToFloat(Integer) (Default|GetAgroRange _asbp_aminion)) (Utilities|Array|MakeArray (Utilities|Enum|LiteralenumEObjectTypeQuery "ObjectTypeQuery3")) false (Utilities|Array|MakeArray _returnvalue) "None"))
  (return _outhits))

(fn CleanHitArray
  (params (ArrayToBeCleaned :type Array%20of%20Hit%20Result%20Structures))
  (for _array_element ArrayToBeCleaned
    (bind _output_get (LocalVariables|SetHit _array_element))
    (if (Utilities|ValidHit _output_get)
      (Utilities|IsValid (.HitActor (Collision|BreakHitResult (LocalVariables|GetHit)))
        (:Is%20Valid
          (if (and (Math|Boolean|NotEqual(Boolean) (Actor|ActorHasTag (.HitActor (Collision|BreakHitResult (LocalVariables|GetHit))) "Projectile") true) (Utilities|IsEnnemy (Variables|/Game/Sources/BP_ABaseCharacter.BP_ABaseCharacter_C|Getteam (Variables|Default|Getminion)) (.HitActor (Collision|BreakHitResult (LocalVariables|GetHit)))))
            (Utilities|Array|Add (LocalVariables|GetOutputArray) (LocalVariables|GetHit))
            (elif (or (Actor|ActorHasTag (.HitActor (Collision|BreakHitResult (LocalVariables|GetHit))) "Projectile") (Math|Boolean|NotEqual(Boolean) (Utilities|IsEnnemy (Variables|/Game/Sources/BP_ABaseCharacter.BP_ABaseCharacter_C|Getteam (Variables|Default|Getminion)) (.HitActor (Collision|BreakHitResult (LocalVariables|GetHit)))) true))
              (Utilities|Array|Add (LocalVariables|GetOutputActorsToIgnore) (.HitActor (Collision|BreakHitResult (LocalVariables|GetHit))))))))))
  (return (LocalVariables|GetOutputArray) (LocalVariables|GetOutputActorsToIgnore)))

(fn SetBlackBoardValues
  (bind _targetactor (Variables|Default|GettargetActor))
  ;[1 1 1] Set BBValue
  (Utilities|IsValid (Variables|Default|GettargetActor)
    (:Is%20Valid
      (LocalVariables|SetState "NewEnumerator2")
      (Class|BTFunctionLibrary|SetBlackboardValueasEnum (Variables|Default|GetMinionState) (LocalVariables|GetState))
      (Class|BTFunctionLibrary|SetBlackboardValueasObject (Variables|Default|GetTargetToFollow) _targetactor)
      (AI|BehaviorTree|SetBlackboardValueasVector (Variables|Default|GetTargetLocation) (Transformation|GetActorLocation _targetactor)))
    (:Is%20Not%20Valid
      (Class|BTFunctionLibrary|SetBlackboardValueasObject (Variables|Default|GetTargetToFollow) (Variables|Default|GettargetActor)))))