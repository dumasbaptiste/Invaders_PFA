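; BP_MinionSpawner spawns lane minions at its location, handing each one its team and patrol route.
; A looping one-second timer from BeginPlay spawns one BP_LaneMinion running BT_Minion, slightly raised, while the MinionsToSpawn counter remains above zero.
; Each minion receives the spawner's team, path and patrol settings, then its BP_AMinionController is linked and initialized.
; Reset refills the counter from MinionsToSpawnMax to allow another batch.
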(event `SpawnMinionServer`
  (if (> (`self.minionsToSpawn`) 0)
    (bind _returnvalue (`AIBlueprintHelperLibrary.SpawnAIFromClass` "/Game/Sources/Minions/LaneMinions/BP_LaneMinion.BP_LaneMinion_C" "/Game/Sources/Minions/BT_Minion.BT_Minion" (`KismetMathLibrary.MakeVector` (.x (`self.K2_GetActorLocation`)) (.y (`self.K2_GetActorLocation`)) (+ (.z (`self.K2_GetActorLocation`)) 100.0)) (`self.K2_GetActorRotation`) true))
    (set `self.minionsToSpawn` (- (`self.minionsToSpawn`) 1))
    (bind _asbp_lane_minion (cast `/Game/Sources/Minions/LaneMinions/BP_LaneMinion` _returnvalue))
    (set `/Game/Sources/BP_ABaseCharacter.team` (`self.team`) _asbp_lane_minion)
    (set `/Game/Sources/Minions/BP_AMinion.patrolPattern` (`self.PatrolPattern`) _asbp_lane_minion)
    (set `/Game/Sources/Minions/BP_AMinion.path` (`self.Path`) _asbp_lane_minion)
    (set `/Game/Sources/Minions/BP_AMinion.patrolMode` (`self.PatrolMode`) _asbp_lane_minion)
    (bind _returnvalue_2 (`AIBlueprintHelperLibrary.GetAIController` _asbp_lane_minion))
    (bind _asbp_aminion_controller (cast `/Game/Sources/Minions/BP_AMinionController` _returnvalue_2))
    (set `/Game/Sources/Minions/BP_AMinionController.AMinion` _asbp_lane_minion _asbp_aminion_controller)
    (`/Game/Sources/Minions/BP_AMinionController.Initialize` _asbp_aminion_controller)))

(event `self.ReceiveBeginPlay`
  (`KismetSystemLibrary.K2_SetTimerDelegate` (delegate `SpawnMinionServer`) 1.0 true))

(event `self.ReceiveActorBeginOverlap`
  (params (OtherActor :type "Actor Object Reference")))

(event `self.ReceiveTick`
  (params (DeltaSeconds :type "Float (single-precision)")))

(fn `Reset`
  (set `self.minionsToSpawn` (`self.minionsToSpawnMax`)))

(fn `UserConstructionScript`)