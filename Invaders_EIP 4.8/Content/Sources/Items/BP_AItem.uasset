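; BP_AItem is an item that stores shop-style info (name, description, image, price, category) and stat bonuses for a player avatar.
; Initialize fills in all stats and info fields, and CompareItem matches items by Id, Category and Type.
; AddStats applies the bonuses and RemoveStats reverses them by adding negated values.
; Both run only on authority and print a cheat warning on clients.
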(fn ConstructionScript)

(fn AddStats
  (params (Player :type BP%20A%20Avatar%20Object%20Reference))
  (LocalVariables|SetAvatar Player)
  (Networking|SwitchHasAuthority
    (:Authority
      (Default|AddMaxHitPoints (LocalVariables|GetAvatar) (Variables|Stats|GetHitPoints))
      (Default|AddEnergeticResistance (LocalVariables|GetAvatar) (Variables|Stats|GetEnergeticResistance))
      (Default|AddPhysicalResistance (LocalVariables|GetAvatar) (Variables|Stats|GetPhysicalResistance))
      (Default|AddPower (LocalVariables|GetAvatar) (Variables|Stats|GetPower))
      (Utilities|FlowControl|Sequence
        (:then_0
          (Default|AddAttackSpeedPercent (LocalVariables|GetAvatar) (Variables|Stats|GetAttackSpeed)))
        (:then_1
          (Default|AddCriticalHitChance (LocalVariables|GetAvatar) (Variables|Stats|GetCriticalChance)))
        (:then_2
          (Default|AddMovementSpeedPercent (LocalVariables|GetAvatar) (Variables|Stats|GetMovementSpeed)))
        (:then_3
          (Default|AddCooldownReduction (LocalVariables|GetAvatar) (Variables|Stats|GetCooldown)))
        (:then_4
          (Default|AddLifesteal (LocalVariables|GetAvatar) (Variables|Stats|GetLifeSteal)))))
    (:Remote
      (Development|PrintString "Are you trying to cheat ? You're on the client" true true "(R=1.000000,G=0.000000,B=0.000000,A=1.000000)"))))

(fn RemoveStats
  (params (Player :type BP%20A%20Avatar%20Object%20Reference))
  (LocalVariables|SetAvatar Player)
  (Networking|SwitchHasAuthority
    (:Authority
      (Default|AddMaxHitPoints (LocalVariables|GetAvatar) (* (Variables|Stats|GetHitPoints) -1))
      (Default|AddEnergeticResistance (LocalVariables|GetAvatar) (* (Variables|Stats|GetEnergeticResistance) -1))
      (Default|AddPhysicalResistance (LocalVariables|GetAvatar) (* (Variables|Stats|GetPhysicalResistance) -1))
      (Default|AddPower (LocalVariables|GetAvatar) (* (Variables|Stats|GetPower) -1))
      (Utilities|FlowControl|Sequence
        (:then_0
          (Default|AddAttackSpeedPercent (LocalVariables|GetAvatar) (* (Variables|Stats|GetAttackSpeed) -1.0)))
        (:then_1
          (Default|AddCriticalHitChance (LocalVariables|GetAvatar) (* (Variables|Stats|GetCriticalChance) -1.0)))
        (:then_2
          (Default|AddMovementSpeedPercent (LocalVariables|GetAvatar) (* (Variables|Stats|GetMovementSpeed) -1.0)))
        (:then_3
          (Default|AddCooldownReduction (LocalVariables|GetAvatar) (* (Variables|Stats|GetCooldown) -1.0)))
        (:then_4
          (Default|AddLifesteal (LocalVariables|GetAvatar) (* (Variables|Stats|GetLifeSteal) -1.0)))))
    (:Remote
      (Development|PrintString "Are you trying to cheat ? You're on the client" true true "(R=1.000000,G=0.000000,B=0.000000,A=1.000000)"))))

(fn Initialize
  (params (HitPoint :type Integer :default 0) (PhysicalResistance :type Integer :default 0) (EnergeticResistance :type Integer :default 0) (Power :type Integer :default 0) (AttackSpeed :type Float%20%28single-precision%29 :default 0.0) (CriticalChance :type Float%20%28single-precision%29 :default 0.0) (Cooldown :type Float%20%28single-precision%29 :default 0.0) (LifeSteal :type Float%20%28single-precision%29 :default 0.0) (MovementSpeed :type Float%20%28single-precision%29 :default 0.0) (Type :type E_ItemType%20Enum :default "NewEnumerator0") (Name :type String) (Description :type String) (Image :type Slate%20Brush%20Structure) (Price :type Integer :default 0) (Id :type Integer :default 0) (Category :type E_ItemCategory%20Enum :default "NewEnumerator0"))
  ;[1 1 1] Stats
  (Utilities|FlowControl|Sequence
    (:then_0
      (Variables|Stats|SetHitPoints HitPoint))
    (:then_1
      (Variables|Stats|SetPhysicalResistance PhysicalResistance))
    (:then_2
      (Variables|Stats|SetEnergeticResistance EnergeticResistance))
    (:then_3
      (Variables|Stats|SetPower Power))
    (:then_4
      (Variables|Stats|SetAttackSpeed AttackSpeed))
    (:then_5
      (Variables|Stats|SetCriticalChance CriticalChance))
    (:then_6
      (Variables|Stats|SetCooldown Cooldown))
    (:then_7
      (Variables|Stats|SetLifeSteal LifeSteal))
    (:then_8
      (Variables|Stats|SetMovementSpeed MovementSpeed))
    (:then_9
      ;[1 1 1] Information
      (Utilities|FlowControl|Sequence
        (:then_0
          (Variables|Information|SetType Type))
        (:then_1
          (Variables|Information|SetName Name))
        (:then_2
          (Variables|Information|SetDescription Description))
        (:then_3
          (Variables|Information|SetImage Image))
        (:then_4
          (Variables|Information|Setprice Price))
        (:then_5
          (Variables|Information|SetId Id))
        (:then_6
          (Variables|Information|SetCategory Category))))))

(fn CompareItem
  (params (ItemToBeCompared :type BP%20A%20Item%20Object%20Reference))
  (Utilities|IsValid ItemToBeCompared
    (:Is%20Valid
      (LocalVariables|SetRet (Math|Boolean|ANDBoolean (== (Variables|BP_AItem_C|GetId ItemToBeCompared) (Variables|Information|GetId)) (== (Variables|BP_AItem_C|GetCategory ItemToBeCompared) (Variables|Information|GetCategory)) (== (Variables|BP_AItem_C|GetType ItemToBeCompared) (Variables|Information|GetType)))))
    (:Is%20Not%20Valid
      _))
  (return (LocalVariables|GetRet)))