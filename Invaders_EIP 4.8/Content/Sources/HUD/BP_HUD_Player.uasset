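; BP_HUD_Player is the player HUD Blueprint that sets up the player's on-screen UI widgets.
; On BeginPlay it creates the main HUD, shop, tab info and capture widgets, stores each and adds it to the viewport.
; All but the main HUD start hidden.
; Getter functions expose the main HUD and shop widgets to other code.
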(event `self.ReceiveBeginPlay`
  (bind _returnvalue (`GameplayStatics.GetPlayerController` 0))
  (bind _shop (`self.Shop`))
  (bind _returnvalue_2 (`|CreateWidget` "/Game/Sources/HUD/WBP_HUD_Player.WBP_HUD_Player_C" _returnvalue))
  (set `self.HUD_Player` _returnvalue_2)
  (`UserWidget.AddToViewport` (`self.HUD_Player`) 0)
  (bind _returnvalue_3 (`|CreateWidget` "/Game/Sources/Shop/WBP_Shop.WBP_Shop_C" _returnvalue))
  (set `self.Shop` _returnvalue_3)
  (`UserWidget.AddToViewport` _shop 0)
  (`Widget.SetVisibility` _shop "Hidden")
  (bind _returnvalue_4 (`|CreateWidget` "/Game/Sources/Tab/WBP_HUD_Tab.WBP_HUD_Tab_C" (`self.GetOwningPlayerController`)))
  (bind _output_get (set `self.TabInfo` _returnvalue_4))
  (`UserWidget.AddToViewport` _output_get 0)
  (`Widget.SetVisibility` _output_get "Hidden")
  (bind _returnvalue_5 (`|CreateWidget` "/Game/Sources/HUD/WBP_Capture.WBP_Capture_C" (`self.GetOwningPlayerController`)))
  (bind _output_get_2 (set `self.CaptureHUD` _returnvalue_5))
  (`UserWidget.AddToViewport` _output_get_2 0)
  (`Widget.SetVisibility` _output_get_2 "Hidden"))

(fn `Get HUD`
  (returns (HUD :type "Widget Object Reference"))
  (return (`self.HUD_Player`)))

(fn `Get Shop`
  (returns (Shop :type "/Game/Sources/Shop/WBP_Shop Object Reference"))
  (return (`self.Shop`)))

(fn `UserConstructionScript`)