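; BP_Headquarters is a capturable team building that switches to the capturing avatar's team.
; Collision overlap gives a BP_AAvatar the building's team through CanICapture and shows the capture HUD; leaving resets it to -1 and hides the HUD.
; Tick accumulates CaptureProgression while OnCapture is true, assigns AvatarTeam after ten seconds, and zeroes progress otherwise.
; OnCapture and AvatarTeam are never set within this Blueprint.
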(event `self.ReceiveBeginPlay`)

(event `self.ReceiveActorBeginOverlap`
  (params (OtherActor :type "Actor Object Reference")))

(event `self.ReceiveTick`
  (params (DeltaSeconds :type "Float (single-precision)"))
  (bind _oncapture (`self.OnCapture`))
  (if _oncapture
    (bind _output_get (set `self.CaptureProgression` (+ (`self.CaptureProgression`) DeltaSeconds)))
    (if (and _oncapture (>= _output_get 10.0))
      (set `self.Team` (`self.AvatarTeam`)))
    (else
      (set `self.CaptureProgression` 0.0))))

(event `self.Collision.OnComponentBeginOverlap`
  (params (OtherActor :type "Actor Object Reference") (OtherComp :type "PrimitiveComponent Object Reference") (OtherBodyIndex :type Integer) (bFromSweep :type Boolean) (SweepResult :type "EngineTypes.HitResult Structure (by ref)"))
  (bind _asbp_aavatar (cast `/Game/Sources/Avatar/BP_AAvatar` OtherActor)
    (:`then`
      (set `/Game/Sources/Avatar/BP_AAvatar.CanICapture` (`KismetMathLibrary.Conv_ByteToInt` (`self.Team`)) _asbp_aavatar)
      (bind _asbp_invaders_controller (cast `/Game/Sources/PlayerController/BP_Invaders_Controller` (`Pawn.GetController` _asbp_aavatar)))
      (bind _asbp_hud_player (cast `/Game/Sources/HUD/BP_HUD_Player` (`PlayerController.GetHUD` _asbp_invaders_controller)))
      (`Widget.SetVisibility` (`/Game/Sources/HUD/BP_HUD_Player.CaptureHUD` _asbp_hud_player) "Visible"))
    (:`CastFailed`
      (`KismetSystemLibrary.PrintString` "Cast Fail"))))

(event `self.Collision.OnComponentEndOverlap`
  (params (OtherActor :type "Actor Object Reference") (OtherComp :type "PrimitiveComponent Object Reference") (OtherBodyIndex :type Integer))
  (bind _asbp_aavatar (cast `/Game/Sources/Avatar/BP_AAvatar` OtherActor))
  (set `/Game/Sources/Avatar/BP_AAvatar.CanICapture` -1 _asbp_aavatar)
  (bind _asbp_invaders_controller (cast `/Game/Sources/PlayerController/BP_Invaders_Controller` (`Pawn.GetController` _asbp_aavatar)))
  (bind _asbp_hud_player (cast `/Game/Sources/HUD/BP_HUD_Player` (`PlayerController.GetHUD` _asbp_invaders_controller)))
  (`Widget.SetVisibility` (`/Game/Sources/HUD/BP_HUD_Player.CaptureHUD` _asbp_hud_player) "Hidden"))

(fn `UserConstructionScript`)