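; Base attack projectile fired by a building, dealing basic-attack damage to an enemy it hits.
; InitializeProjectile stores the owning building, range and total duration.
; On hit, it damages only the first hit target, if on another team, using the building's power, then flags itself for auto-destruction.
; Finish calls the parent logic and sets the same auto-destroy flag.
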(event `self.ReceiveBeginPlay`)

(event `self.ReceiveActorBeginOverlap`
  (params (OtherActor :type "Actor Object Reference")))

(event `self.ReceiveTick`
  (params (DeltaSeconds :type "Float (single-precision)"))
  (`parent.ReceiveTick` 0.0))

(fn `Finish`
  (returns (return :type Boolean))
  (`parent.Finish`)
  (bind _output_get (set `self.bAutoDestroyWhenFinished` true))
  (return _output_get))

(fn `InitializeProjectile`
  (params (Duration :type "Float (double-precision)" :default 0.0) (Range :type Integer :default 0) (Owner :type "/Game/Sources/Buildings/BP_ABuilding Object Reference"))
  (set `self.totalDuration` Duration)
  (set `self.range` Range)
  (set `self.OwnerBuilding` Owner))

(fn `OnHit`
  (returns (return :type Boolean))
  (bind _hitten (`self.hitten`))
  (bind _ownerbuilding (`self.OwnerBuilding`))
  (bind _item (`KismetArrayLibrary.Array_Get` _hitten))
  (`parent.OnHit`)
  (`/Engine/EditorBlueprintResources/StandardMacros.IsValid` _ownerbuilding
    (:`Is Valid`
      (if (> (`KismetArrayLibrary.Array_Length` _hitten) 0)
        (if (!= (`/Game/Sources/Buildings/BP_ABuilding.GetTeam` _ownerbuilding) (`/Game/Sources/BP_ABaseCharacter.team` _item))
          (`/Game/Sources/BP_ABaseCharacter.TakeDamages` _item false "NewEnumerator0" true (`/Game/Sources/Buildings/BP_ABuilding.GetPower` (`self.OwnerBuilding`)) null)
          (set `self.bAutoDestroyWhenFinished` true))
        (return false)))))

(fn `UserConstructionScript`
  (`parent.UserConstructionScript`))