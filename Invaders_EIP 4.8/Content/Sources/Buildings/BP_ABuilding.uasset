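; BP_ABuilding is a building Blueprint, apparently a base class, that holds combat stats and can fire on a target.
; Getters and setters expose hit points, attack speed, resistances and power, while team and range have getters only.
; Attack spawns a scaled-down BP_BuildingBaseAttackProjectile at ProjectileSpawn, aimed at the target and initialized with range and owner.
; Range has an empty RepNotify, and the event graph holds no logic.
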(event `self.ReceiveBeginPlay`)

(event `self.ReceiveActorBeginOverlap`
  (params (OtherActor :type "Actor Object Reference")))

(event `self.ReceiveTick`
  (params (DeltaSeconds :type "Float (single-precision)")))

(fn `Attack`
  (params (Target :type "Actor Object Reference"))
  (bind _returnvalue (`|SpawnActorFromClass` "/Game/Sources/Buildings/BP_BuildingBaseAttackProjectile.BP_BuildingBaseAttackProjectile_C" (`KismetMathLibrary.MakeTransform` (`SceneComponent.K2_GetComponentLocation` (`self.ProjectileSpawn`)) (`KismetMathLibrary.FindLookAtRotation` (`SceneComponent.K2_GetComponentLocation` (`self.ProjectileSpawn`)) (`self.K2_GetActorLocation` Target)) (0.1 0.1 0.1)) true))
  (`/Game/Sources/Buildings/BP_BuildingBaseAttackProjectile.InitializeProjectile` _returnvalue 0.1 (`self.range`) self))

(fn `GetAttackSpeed`
  (returns (Amount :type "Float (double-precision)"))
  (return (`self.AttackSpeed`)))

(fn `GetEnergyResistance`
  (returns (Amount :type Integer))
  (return (`self.EnergyResistance`)))

(fn `GetHitPoint`
  (returns (Amount :type Integer))
  (return (`self.HitPoint`)))

(fn `GetPhysicalResistance`
  (returns (Amount :type Integer))
  (return (`self.PhysicalResistance`)))

(fn `GetPower`
  (returns (Amount :type Integer))
  (return (`self.Power`)))

(fn `GetRange`
  (returns (NewParam :type Integer))
  (return (`self.Range`)))

(fn `GetTeam`
  (returns (Team :type "/Game/Sources/E_Team Enum"))
  (return (`self.Team`)))

(fn `OnRep_Range`)

(fn `SetAttackSpeed`
  (params (Amount :type "Float (double-precision)" :default 0.0))
  (set `self.AttackSpeed` Amount))

(fn `SetEnergyResistance`
  (params (Amount :type Integer :default 0))
  (set `self.EnergyResistance` Amount))

(fn `SetHitPoint`
  (params (Amount :type Integer :default 0))
  (set `self.HitPoint` Amount))

(fn `SetPhysicalResistance`
  (params (Amount :type Integer :default 0))
  (set `self.PhysicalResistance` Amount))

(fn `SetPower`
  (params (Power :type Integer :default 0))
  (set `self.Power` Power))

(fn `UserConstructionScript`)