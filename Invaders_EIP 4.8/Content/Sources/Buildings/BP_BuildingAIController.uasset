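; BP_BuildingAIController is the AI controller for buildings, starting their behavior tree when it possesses one.
; On possess it calls Initialize, which sets up the BB_Building blackboard and resets the AttackCooldown key to zero.
; It then runs BT_Building and prints a debug message, leaving all decision logic to the tree.
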(event EventBeginPlay)

(event EventTick
  (params (DeltaSeconds :type Float%20%28single-precision%29)))

(event EventOnPossess
  (params (PossessedPawn :type Pawn%20Object%20Reference))
  (CallFunction|Initialize))

(fn ConstructionScript)

(fn Initialize
  (bind _returnvalue (Class|AIController|UseBlackboard "/Game/Sources/Buildings/BB_Building.BB_Building"))
  (if _returnvalue
    (LocalVariables|SetKeyName "AttackCooldown")
    (AI|Components|Blackboard|SetValueasFloat (AI|GetBlackboard self) (LocalVariables|GetKeyName) 0.0)
    (AI|RunBehaviorTree "/Game/Sources/Buildings/BT_Building.BT_Building")
    (Development|PrintString "Initialized")))