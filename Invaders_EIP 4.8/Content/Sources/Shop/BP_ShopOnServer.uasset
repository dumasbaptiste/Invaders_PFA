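; Server-side shop actor that holds the item catalogue and creates items sold to players.
; On BeginPlay, Initialize spawns one instance of every configured item class in each category, from stats like Power and Life Steal to Usable, into per-category arrays.
; GetItem searches those instances by category and ID to resolve the class.
; SellItemToPlayer then spawns a fresh copy at the world origin and returns it, without any payment check.
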(event EventBeginPlay
  (CallFunction|Initialize))

(fn ConstructionScript)

(fn SellItemtoPlayer
  (params (ItemID :type Integer :default 0) (ItemType :type E_ItemType%20Enum) (ItemCategory :type E_ItemCategory%20Enum :default "NewEnumerator0"))
  (bind (_itemactor _itemclass _isvalid) (CallFunction|GetItem ItemCategory ItemID))
  (if _isvalid
    (bind _returnvalue (Game|SpawnActorfromClass _itemclass (Math|Transform|MakeTransform "0, 0, 0") false 0))
    (LocalVariables|SetRet _returnvalue))
  (return (LocalVariables|GetRet)))

(fn GetItemClassesbyCategory
  (params (Category :type E_ItemCategory%20Enum :default "NewEnumerator0"))
  (switch Utilities|FlowControl|Switch|SwitchonE_ItemCategory Category
    (:NewEnumerator0
      (LocalVariables|SetItemsArray (Variables|ItemCategoryClasses|GetPowerItemClasses)))
    (:NewEnumerator1
      (LocalVariables|SetItemsArray (Variables|ItemCategoryClasses|GetAttackSpeedItemClasses)))
    (:NewEnumerator2
      (LocalVariables|SetItemsArray (Variables|ItemCategoryClasses|GetCriticalHitClasses)))
    (:NewEnumerator3
      (LocalVariables|SetItemsArray (Variables|ItemCategoryClasses|GetHitPointItemClasses)))
    (:NewEnumerator4
      (LocalVariables|SetItemsArray (Variables|ItemCategoryClasses|GetPhysicalResistanceItemClasses)))
    (:NewEnumerator5
      (LocalVariables|SetItemsArray (Variables|ItemCategoryClasses|GetEnergyResistanceItemClasses)))
    (:NewEnumerator6
      (LocalVariables|SetItemsArray (Variables|ItemCategoryClasses|GetMouvementSpeedItemClasses)))
    (:NewEnumerator7
      (LocalVariables|SetItemsArray (Variables|ItemCategoryClasses|GetLifeStealItemClasses)))
    (:NewEnumerator8
      (LocalVariables|SetItemsArray (Variables|ItemCategoryClasses|GetCooldownItemClasses)))
    (:NewEnumerator9
      (LocalVariables|SetItemsArray (Variables|ItemCategoryClasses|GetUsableItemClasses))))
  (return (LocalVariables|GetItemsArray)))

(fn GetItem
  (params (ItemCategory :type E_ItemCategory%20Enum :default "NewEnumerator0") (ItemID :type Integer :default 0))
  (LocalVariables|SetID ItemID)
  (switch Utilities|FlowControl|Switch|SwitchonE_ItemCategory ItemCategory
    (:NewEnumerator0
      (bind _array_element (Utilities|Array|ForEachLoopwithBreak (Variables|ItemCategoryActors|GetPowerItems) :!label _label)
        (:LoopBody
          (bind _output_get (LocalVariables|SetCurrentItem _array_element))
          (if (== (Variables|/Game/Sources/Items/BP_AItem.BP_AItem_C|GetId _output_get) (LocalVariables|GetID))
            (goto _label Break)))
        (:Completed
          (bind _output_get_2 (LocalVariables|SetValid (Utilities|IsValid (LocalVariables|GetCurrentItem)) :!label _label_2))
          (return (LocalVariables|GetCurrentItem) (.AsBP%20AItem (Utilities|Casting|CastToBP_AItemClass (Utilities|GetClass (LocalVariables|GetCurrentItem)))) (and _output_get_2 (.bSuccess (Utilities|Casting|CastToBP_AItemClass (Utilities|GetClass (LocalVariables|GetCurrentItem)))))))))
    (:NewEnumerator1
      (bind _array_element_2 (Utilities|Array|ForEachLoopwithBreak (Variables|ItemCategoryActors|GetAttackSpeedItems) :!label _label_3)
        (:LoopBody
          (bind _output_get_3 (LocalVariables|SetCurrentItem _array_element_2))
          (if (== (Variables|/Game/Sources/Items/BP_AItem.BP_AItem_C|GetId _output_get_3) (LocalVariables|GetID))
            (goto _label_3 Break)))
        (:Completed
          (goto _label_2))))
    (:NewEnumerator2
      (bind _array_element_3 (Utilities|Array|ForEachLoopwithBreak (Variables|ItemCategoryActors|GetCriticalHitItems) :!label _label_4)
        (:LoopBody
          (bind _output_get_4 (LocalVariables|SetCurrentItem _array_element_3))
          (if (== (Variables|/Game/Sources/Items/BP_AItem.BP_AItem_C|GetId _output_get_4) (LocalVariables|GetID))
            (goto _label_4 Break)))
        (:Completed
          (goto _label_2))))
    (:NewEnumerator3
      (bind _array_element_4 (Utilities|Array|ForEachLoopwithBreak (Variables|ItemCategoryActors|GetHitPointItems) :!label _label_5)
        (:LoopBody
          (bind _output_get_5 (LocalVariables|SetCurrentItem _array_element_4))
          (if (== (Variables|/Game/Sources/Items/BP_AItem.BP_AItem_C|GetId _output_get_5) (LocalVariables|GetID))
            (goto _label_5 Break)))
        (:Completed
          (goto _label_2))))
    (:NewEnumerator4
      (bind _array_element_5 (Utilities|Array|ForEachLoopwithBreak (Variables|ItemCategoryActors|GetPhysicalResistanceItems) :!label _label_6)
        (:LoopBody
          (bind _output_get_6 (LocalVariables|SetCurrentItem _array_element_5))
          (if (== (Variables|/Game/Sources/Items/BP_AItem.BP_AItem_C|GetId _output_get_6) (LocalVariables|GetID))
            (goto _label_6 Break)))
        (:Completed
          (goto _label_2))))
    (:NewEnumerator5
      (bind _array_element_6 (Utilities|Array|ForEachLoopwithBreak (Variables|ItemCategoryActors|GetEnergyResistanceItems) :!label _label_7)
        (:LoopBody
          (bind _output_get_7 (LocalVariables|SetCurrentItem _array_element_6))
          (if (== (Variables|/Game/Sources/Items/BP_AItem.BP_AItem_C|GetId _output_get_7) (LocalVariables|GetID))
            (goto _label_7 Break)))
        (:Completed
          (goto _label_2))))
    (:NewEnumerator6
      (bind _array_element_7 (Utilities|Array|ForEachLoopwithBreak (Variables|ItemCategoryActors|GetMouvementSpeedItems) :!label _label_8)
        (:LoopBody
          (bind _output_get_8 (LocalVariables|SetCurrentItem _array_element_7))
          (if (== (Variables|/Game/Sources/Items/BP_AItem.BP_AItem_C|GetId _output_get_8) (LocalVariables|GetID))
            (goto _label_8 Break)))
        (:Completed
          (goto _label_2))))
    (:NewEnumerator7
      (bind _array_element_8 (Utilities|Array|ForEachLoopwithBreak (Variables|ItemCategoryActors|GetLifeStealItems) :!label _label_9)
        (:LoopBody
          (bind _output_get_9 (LocalVariables|SetCurrentItem _array_element_8))
          (if (== (Variables|/Game/Sources/Items/BP_AItem.BP_AItem_C|GetId _output_get_9) (LocalVariables|GetID))
            (goto _label_9 Break)))
        (:Completed
          (goto _label_2))))
    (:NewEnumerator8
      (bind _array_element_9 (Utilities|Array|ForEachLoopwithBreak (Variables|ItemCategoryActors|GetCooldownItems) :!label _label_10)
        (:LoopBody
          (bind _output_get_10 (LocalVariables|SetCurrentItem _array_element_9))
          (if (== (Variables|/Game/Sources/Items/BP_AItem.BP_AItem_C|GetId _output_get_10) (LocalVariables|GetID))
            (goto _label_10 Break)))
        (:Completed
          (goto _label_2))))
    (:NewEnumerator9
      (bind _array_element_10 (Utilities|Array|ForEachLoopwithBreak (Variables|ItemCategoryActors|GetUsableItems) :!label _label_11)
        (:LoopBody
          (bind _output_get_11 (LocalVariables|SetCurrentItem _array_element_10))
          (if (== (Variables|/Game/Sources/Items/BP_AItem.BP_AItem_C|GetId _output_get_11) (LocalVariables|GetID))
            (goto _label_11 Break)))
        (:Completed
          (goto _label_2))))))

(fn Initialize
  (bind _enumvalue (|ForEachE_ItemCategory)
    (:LoopBody
      (bind _output_get (LocalVariables|SetCurrentCategory _enumvalue))
      (for _array_element (NewEnumerator0|GetItemClassesbyCategory _output_get)
        (bind _returnvalue (Game|SpawnActorfromClass _array_element (Math|Transform|MakeTransform "0, 0, 0") false 0))
        (LocalVariables|SetItem _returnvalue)
        (switch Utilities|FlowControl|Switch|SwitchonE_ItemCategory (LocalVariables|GetCurrentCategory)
          (:NewEnumerator0
            (Utilities|Array|Add (Variables|ItemCategoryActors|GetPowerItems) (LocalVariables|GetItem)))
          (:NewEnumerator1
            (Utilities|Array|Add (Variables|ItemCategoryActors|GetAttackSpeedItems) (LocalVariables|GetItem)))
          (:NewEnumerator2
            (Utilities|Array|Add (Variables|ItemCategoryActors|GetCriticalHitItems) (LocalVariables|GetItem)))
          (:NewEnumerator3
            (Utilities|Array|Add (Variables|ItemCategoryActors|GetHitPointItems) (LocalVariables|GetItem)))
          (:NewEnumerator4
            (Utilities|Array|Add (Variables|ItemCategoryActors|GetPhysicalResistanceItems) (LocalVariables|GetItem)))
          (:NewEnumerator5
            (Utilities|Array|Add (Variables|ItemCategoryActors|GetEnergyResistanceItems) (LocalVariables|GetItem)))
          (:NewEnumerator6
            (Utilities|Array|Add (Variables|ItemCategoryActors|GetMouvementSpeedItems) (LocalVariables|GetItem)))
          (:NewEnumerator7
            (Utilities|Array|Add (Variables|ItemCategoryActors|GetLifeStealItems) (LocalVariables|GetItem)))
          (:NewEnumerator8
            (Utilities|Array|Add (Variables|ItemCategoryActors|GetCooldownItems) (LocalVariables|GetItem)))
          (:NewEnumerator9
            (Utilities|Array|Add (Variables|ItemCategoryActors|GetUsableItems) (LocalVariables|GetItem))))))))